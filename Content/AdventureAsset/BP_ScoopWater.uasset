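; BP_ScoopWater is a world interaction actor that turns into a BP_CRAdventureWaterItem when scooped.
; Box overlap with BP_CRAdventureCharacter sets the Scoop flag and enables input for player 0; leaving clears the flag but keeps input enabled.
; Pressing F while Scoop is true spawns the water item at the actor's location and destroys the actor.
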(event `Key|F`
  (params (Key :type "Key Structure"))
  (:`Pressed`
    (if (stale `self.Box.OnComponentBeginOverlap` _output_get)
      (`|SpawnActorFromClass` "/Game/CosmicRestaurant/Blueprints/Item/BP_CRAdventureWaterItem.BP_CRAdventureWaterItem_C" (`KismetMathLibrary.MakeTransform` (`self.K2_GetActorLocation`)) "Undefined" "MultiplyWithRoot" null null)
      (`self.K2_DestroyActor`))))

(event `self.Box.OnComponentBeginOverlap`
  (params (OverlappedComponent :type "PrimitiveComponent Object Reference") (OtherActor :type "Actor Object Reference") (OtherComp :type "PrimitiveComponent Object Reference") (OtherBodyIndex :type Integer) (bFromSweep :type Boolean) (SweepResult :type "HitResult Structure (by ref)"))
  (cast `/Game/CosmicRestaurant/Blueprints/Character/BP_CRAdventureCharacter` OtherActor)
  (bind _output_get (set `self.Scoop?` true))
  (`self.EnableInput` (`GameplayStatics.GetPlayerController` 0)))

(event `self.Box.OnComponentEndOverlap`
  (params (OverlappedComponent :type "PrimitiveComponent Object Reference") (OtherActor :type "Actor Object Reference") (OtherComp :type "PrimitiveComponent Object Reference") (OtherBodyIndex :type Integer))
  (cast `/Game/CosmicRestaurant/Blueprints/Character/BP_CRAdventureCharacter` OtherActor)
  (set `self.Scoop?` false))

(fn `UserConstructionScript`)