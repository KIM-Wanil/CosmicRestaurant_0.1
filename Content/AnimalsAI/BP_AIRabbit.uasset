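; BP_AIRabbit is an animal AI that flees from the player and turns into a steak when hit by a rock.
; Pawn sensing stores the sighted adventure character and starts RunAwayAi, which moves to a random reachable point around a spot directly away from it.
; The move re-triggers itself on success or failure, so fleeing never ends once started.
; A capsule hit from a Rock-tagged actor spawns BP_Steak and destroys the rabbit.
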(event `self.PawnSensing.OnSeePawn`
  (params (Pawn :type "Pawn Object Reference"))
  (bind _ascradventure_character (cast `CRAdventureCharacter` Pawn))
  (set `self.As CRAdventure Character` _ascradventure_character)
  (`self.RunAwayAi`))

(event `RunAwayAi`
  (bind _returnvalue (`self.K2_GetActorLocation`))
  (`|AIMoveTo` self (`NavigationSystemV1.K2_GetRandomReachablePointInRadius` (`KismetMathLibrary.MakeVector` (.x (+ _returnvalue (* (`KismetMathLibrary.GetForwardVector` (`KismetMathLibrary.FindLookAtRotation` _returnvalue (`self.K2_GetActorLocation` (`self.As CRAdventure Character`)))) -500.0))) (.y (+ _returnvalue (* (`KismetMathLibrary.GetForwardVector` (`KismetMathLibrary.FindLookAtRotation` _returnvalue (`self.K2_GetActorLocation` (`self.As CRAdventure Character`)))) -500.0))) (.z _returnvalue)) 500.0 null null) null
    (:`OnSuccess`
      _)
    (:`OnFail`
      _))
  (`self.RunAwayAi`))

(event `self.Capsule.OnComponentHit`
  (params (HitComponent :type "PrimitiveComponent Object Reference") (OtherActor :type "Actor Object Reference") (OtherComp :type "PrimitiveComponent Object Reference") (NormalImpulse :type "Vector Structure") (Hit :type "HitResult Structure (by ref)"))
  (if (`self.ActorHasTag` OtherActor "Rock")
    (`|SpawnActorFromClass` "/Game/CosmicRestaurant/Blueprints/Adventure/Hunting/BP_Steak.BP_Steak_C" (`KismetMathLibrary.MakeTransform` (`self.K2_GetActorLocation`)) "Undefined" "MultiplyWithRoot" null null)
    (`self.K2_DestroyActor`)))

(fn `UserConstructionScript`)