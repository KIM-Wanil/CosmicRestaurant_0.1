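; BP_AIWolf is an AI wolf that detects the player, can bite and drops a steak when killed by a rock.
; PawnSensing sets the HasSeenPlayer blackboard key when it sees a BP_CRAdventureCharacter, and nothing here clears it.
; A capsule hit from an actor tagged Rock spawns BP_Steak at the wolf's location and destroys the wolf.
; The Attack event only plays the bite montage, with no damage logic.
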(event `self.PawnSensing.OnSeePawn`
  (params (Pawn :type "Pawn Object Reference"))
  (cast `/Game/CosmicRestaurant/Blueprints/Character/BP_CRAdventureCharacter` Pawn)
  (`BlackboardComponent.SetValueAsBool` (`AIBlueprintHelperLibrary.GetBlackboard` (`AIBlueprintHelperLibrary.GetAIController` self)) "HasSeenPlayer" true))

(event `self.Capsule.OnComponentHit`
  (params (HitComponent :type "PrimitiveComponent Object Reference") (OtherActor :type "Actor Object Reference") (OtherComp :type "PrimitiveComponent Object Reference") (NormalImpulse :type "Vector Structure") (Hit :type "HitResult Structure (by ref)"))
  (if (`self.ActorHasTag` OtherActor "Rock")
    (`|SpawnActorFromClass` "/Game/CosmicRestaurant/Blueprints/Adventure/Hunting/BP_Steak.BP_Steak_C" (`KismetMathLibrary.MakeTransform` (`self.K2_GetActorLocation`)) "Undefined" "MultiplyWithRoot" null null)
    (`self.K2_DestroyActor`)))

(event `Attack`
  (`|PlayMontage` (`self.Mesh`) "/Game/UsedAssets/Wolf/Animations/ANIM_WolfBie.ANIM_WolfBie"))

(fn `UserConstructionScript`)