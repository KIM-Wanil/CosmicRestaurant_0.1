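; BP_Steak is a gatherable steak in the adventure hunting content that the player removes by pressing F while nearby.
; Capsule overlap sets a Gather flag and enables player input, while end overlap clears only the flag.
; Tick feeds the flag into the BPPlants custom depth toggle, likely for highlighting.
; F destroys the actor when the flag is set, without granting any item here.
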(event `self.ReceiveTick`
  (params (DeltaSeconds :type "Float (single-precision)"))
  (`PrimitiveComponent.SetRenderCustomDepth` (`self.BP_Plants`) (`self.Gather`)))

(event `Key|F`
  (params (Key :type "Key Structure"))
  ;[1 1 1] Actor Destroy
  (:`Pressed`
    (if (stale `self.Capsule.OnComponentBeginOverlap` _output_get)
      (`self.K2_DestroyActor`))))

(event `self.Capsule.OnComponentBeginOverlap`
  (params (OverlappedComponent :type "PrimitiveComponent Object Reference") (OtherActor :type "Actor Object Reference") (OtherComp :type "PrimitiveComponent Object Reference") (OtherBodyIndex :type Integer) (bFromSweep :type Boolean) (SweepResult :type "HitResult Structure (by ref)"))
  ;[1 1 1] Actor Destroy
  (bind _output_get (set `self.Gather` true))
  (`self.EnableInput` (`GameplayStatics.GetPlayerController` 0)))

(event `self.Capsule.OnComponentEndOverlap`
  (params (OverlappedComponent :type "PrimitiveComponent Object Reference") (OtherActor :type "Actor Object Reference") (OtherComp :type "PrimitiveComponent Object Reference") (OtherBodyIndex :type Integer))
  ;[1 1 1] Actor Destroy
  (set `self.Gather` false))

(fn `UserConstructionScript`)