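; Big monster AI character for Cosmic Restaurant's adventure mode that kills the player on contact with a jumpscare.
; On BeginPlay it sets its movement speed from GetAIWalkSpeed.
; When its catch capsule overlaps the adventure character, a one-shot sequence disables input, hides the monster mesh and plays the jumpscare on the player's own component with its light shown.
; After a short delay it shows WB_Death and flags IsDead in GI_Inventory.
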(event `self.ReceiveBeginPlay`
  (bind _returnvalue (`self.GetAIWalkSpeed`))
  (set `CharacterMovementComponent.MaxWalkSpeed` _returnvalue (`self.CharacterMovement`)))

(event `self.Catchcapsule.OnComponentBeginOverlap`
  (params (OverlappedComponent :type "PrimitiveComponent Object Reference") (OtherActor :type "Actor Object Reference") (OtherComp :type "PrimitiveComponent Object Reference") (OtherBodyIndex :type Integer) (bFromSweep :type Boolean) (SweepResult :type "HitResult Structure (by ref)"))
  (bind _asbp_cradventure_character (cast `/Game/CosmicRestaurant/Blueprints/Character/BP_CRAdventureCharacter` OtherActor))
  (`/Engine/EditorBlueprintResources/StandardMacros.DoOnce` false
    (:`Completed`
      (`self.DisableInput` _asbp_cradventure_character null)
      (bind _jumpscare (`/Game/CosmicRestaurant/Blueprints/Character/BP_CRAdventureCharacter.Jumpscare` _asbp_cradventure_character))
      (`SceneComponent.SetVisibility` _jumpscare true false)
      (`SceneComponent.SetVisibility` (`self.Mesh`) false false)
      (`SceneComponent.SetVisibility` (`/Game/CosmicRestaurant/Blueprints/Character/BP_CRAdventureCharacter.LightCom` _asbp_cradventure_character) true false)
      (`SkeletalMeshComponent.PlayAnimation` _jumpscare "/Game/TwigPeople/Animations/AM_JumpScare.AM_JumpScare" false)
      (`KismetSystemLibrary.Delay` 0.8)
      (bind _returnvalue (`|CreateWidget` "/Game/Widget/WB_Death.WB_Death_C" (`GameplayStatics.GetPlayerController` 0)))
      (`UserWidget.AddToViewport` _returnvalue 0)
      (bind _asgi_inventory (cast `/Game/CosmicRestaurant/Blueprints/GI_Inventory` (`GameplayStatics.GetGameInstance`)))
      (set `/Game/CosmicRestaurant/Blueprints/GI_Inventory.bIsDead` true _asgi_inventory))))

(fn `UserConstructionScript`)