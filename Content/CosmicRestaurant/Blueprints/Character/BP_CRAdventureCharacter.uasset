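; First-person player character for Cosmic Restaurant's adventure mode, handling gathering, rock throwing, sprint stamina and a timed flashlight.
; Holding F in the CanGatherItem state adds the traced item to the inventory component, saves through GI_Inventory and briefly shows item info.
; Sprinting drains stamina with camera shake and releasing regenerates it, both via RetriggerableDelay loops.
; Tick tracks hold time and drains flashlight time, which never refills here.
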(event `OffItemInfo`
  (set `/Game/CosmicRestaurant/Blueprints/UI/Gaeun_Folder/Adventure/UI_Adventure_Info.bItemInfo` false (`self.InfoUI`)))

(event `self.ReceiveBeginPlay`
  (bind _returnvalue (`GameplayStatics.GetPlayerController` 0))
  (`|ExecutionSequence`
    (:`then_0`
      (bind _returnvalue_2 (`|CreateWidget` "/Game/Widget/W_DotHud.W_DotHud_C" _returnvalue))
      (`UserWidget.AddToViewport` _returnvalue_2 0))
    (:`then_1`
      (bind _returnvalue_3 (`|CreateWidget` "/Game/CosmicRestaurant/Blueprints/UI/Gaeun_Folder/Adventure/UI_Adventure_.UI_Adventure__C" _returnvalue))
      (`UserWidget.AddToViewport` _returnvalue_3 0))
    (:`then_2`
      (bind _returnvalue_4 (`|CreateWidget` "/Game/CosmicRestaurant/Blueprints/UI/Gaeun_Folder/Adventure/UI_Adventure_Info.UI_Adventure_Info_C" _returnvalue))
      (`UserWidget.AddToViewport` _returnvalue_4 0)
      (set `self.InfoUI` _returnvalue_4))
    (:`then_3`
      (bind _asgi_inventory (cast `/Game/CosmicRestaurant/Blueprints/GI_Inventory` (`GameplayStatics.GetGameInstance`)))
      (`/Game/CosmicRestaurant/Blueprints/GI_Inventory.LoadInventoryData` _asgi_inventory (`/Game/CosmicRestaurant/Blueprints/UI/Gaeun_Folder/Inventory/Inventory_Wanil/BP_Inventory_Wanil.Content2` (`self.BP_Inventory_Wanil`))))
    (:`then_4`
      (set `self.RemainFlashTime` (`self.MaxFlashTime`)))))

(event `self.ReceiveTick`
  (params (DeltaSeconds :type "Float (single-precision)"))
  (bind _infoui (`self.InfoUI`))
  (`|ExecutionSequence`
    (:`then_0`
      (if (`self.bIsHold`)
        (bind _output_get (set `self.HeldTime` (`PlayerController.GetInputKeyTimeDown` (`GameplayStatics.GetPlayerController` 0) "F")))
        (`KismetSystemLibrary.PrintString` (`KismetStringLibrary.Conv_DoubleToString` _output_get))
        (if (>= (`self.HeldTime`) (`self.MaxHeldTime`))
          (`self.GatherItem`)
          (`GameplayStatics.PlaySound2D` "/Game/CosmicRestaurant/Sound/SW_ItemGet.SW_ItemGet" 1.0 1.0 0.0 null null)
          (set `self.bIsHold` false)
          (set `/Game/CosmicRestaurant/Blueprints/UI/Gaeun_Folder/Adventure/UI_Adventure_Info.bActionInfo` false _infoui)
          (set `/Game/CosmicRestaurant/Blueprints/UI/Gaeun_Folder/Adventure/UI_Adventure_Info.bItemInfo` true _infoui)
          (`KismetSystemLibrary.K2_SetTimerDelegate` (delegate `OffItemInfo`) 1.0))))
    (:`then_1`
      (if (`self.bFlash`)
        (bind _output_get_2 (set `self.RemainFlashTime` (- (`self.RemainFlashTime`) (* DeltaSeconds 1.0))))
        (if (<= _output_get_2 0.0)
          (`SceneComponent.SetVisibility` (`self.SpotLight`) false false)
          (set `self.bFlash` false))))))

(event `Key|F`
  (params (Key :type "Key Structure"))
  ;[1 1 1] 아이템 인벤토리 추가
  (:`Pressed`
    (if (`|EnumEquality` (`self.CurrentState`) "CanGatherItem")
      (set `self.bIsHold` true)
      (set `/Game/CosmicRestaurant/Blueprints/UI/Gaeun_Folder/Adventure/UI_Adventure_Info.bActionInfo` true (`self.InfoUI`))
      (`GameplayStatics.PlaySound2D` "/Game/CosmicRestaurant/Sound/SW_Gathering.SW_Gathering" 1.0 1.0 0.0 null null)))
  (:`Released`
    (set `self.bIsHold` false)
    (set `/Game/CosmicRestaurant/Blueprints/UI/Gaeun_Folder/Adventure/UI_Adventure_Info.bActionInfo` false (`self.InfoUI`))))

(event `EnhancedInput|/Game/CosmicRestaurant/Input/Actions/IA_Throw`
  (params (ActionValue :type Boolean) (ElapsedSeconds :type "Float (double-precision)") (TriggeredSeconds :type "Float (double-precision)") (InputAction :type "InputAction Object Reference" :default "/Game/CosmicRestaurant/Input/Actions/IA_Throw.IA_Throw"))
  (bind (_returnvalue_location _returnvalue_rotation) (`KismetMathLibrary.BreakTransform` (`SceneComponent.K2_GetComponentToWorld` (`self.FirstPersonCameraComponent`))))
  (:`Triggered`
    (`|PlayMontage` (`self.Mesh`) "/Game/UsedAssets/CommonResource/FirstPersonArms/Animations/FP_Rifle_Shoot_Montage.FP_Rifle_Shoot_Montage"
      (:`then`
        (`|SpawnActorFromClass` "/Game/CosmicRestaurant/Blueprints/Adventure/Hunting/BP_ThrowRock.BP_ThrowRock_C" (`KismetMathLibrary.MakeTransform` _returnvalue_location _returnvalue_rotation) "AdjustIfPossibleButAlwaysSpawn" "MultiplyWithRoot" null null)))))

(event `GatherItem`
  (bind _bp_inventory_wanil (`self.BP_Inventory_Wanil`))
  (bind _traceditem (`self.TracedItem`))
  ;[1 1 1] 아이템 인벤토리 추가
  (if (`KismetSystemLibrary.IsValid` _traceditem)
    (bind _asbp_cradventure_item_base (cast `/Game/CosmicRestaurant/Blueprints/Item/BP_CRAdventureItemBase` _traceditem))
    (bind _itemdatacom_wanil (`/Game/CosmicRestaurant/Blueprints/Item/BP_CRAdventureItemBase.ItemDataCom_Wanil` _asbp_cradventure_item_base))
    (bind (_itemid_datatable _itemid_rowname) (break `DataTableRowHandle` (`/Game/CosmicRestaurant/Blueprints/UI/Gaeun_Folder/Inventory/Inventory_Wanil/ItemDataCom_Wanil.ItemID` _itemdatacom_wanil)))
    (bind (_success _quantityremaining) (`/Game/CosmicRestaurant/Blueprints/UI/Gaeun_Folder/Inventory/Inventory_Wanil/BP_Inventory_Wanil.AddToInventory` _bp_inventory_wanil _itemid_rowname (`/Game/CosmicRestaurant/Blueprints/UI/Gaeun_Folder/Inventory/Inventory_Wanil/ItemDataCom_Wanil.Quantity` _itemdatacom_wanil)))
    (set `/Game/CosmicRestaurant/Blueprints/UI/Gaeun_Folder/Adventure/UI_Adventure_Info.EarnedItemName` (`KismetTextLibrary.Conv_NameToText` _itemid_rowname) (`self.InfoUI`))
    (`KismetSystemLibrary.PrintText` (`|FormatText` "Name : {name} , Quantity : {quantity}" _itemid_rowname _quantityremaining))
    (`self.K2_DestroyActor` _asbp_cradventure_item_base)
    (bind _asgi_inventory (cast `/Game/CosmicRestaurant/Blueprints/GI_Inventory` (`GameplayStatics.GetGameInstance`)))
    (`/Game/CosmicRestaurant/Blueprints/GI_Inventory.SaveInventoryData` _asgi_inventory (`/Game/CosmicRestaurant/Blueprints/UI/Gaeun_Folder/Inventory/Inventory_Wanil/BP_Inventory_Wanil.Content2` _bp_inventory_wanil))))

(event `Key|LeftShift`
  (params (Key :type "Key Structure"))
  (bind _charactermovement (`self.CharacterMovement`))
  ;[1 1 1] Stamina
  (:`Pressed`
    (set `self.CanIncreaseStamina?` false)
    (set `self.bIsRun` true)
    (set `CharacterMovementComponent.MaxWalkSpeed` 1200.0 _charactermovement :!label _label)
    (`KismetSystemLibrary.RetriggerableDelay` 0.2)
    (`self.UseStamina`)
    (if (`self.bIsRun`)
      (goto _label)))
  (:`Released`
    (set `self.bIsRun` false)
    (set `CharacterMovementComponent.MaxWalkSpeed` 600.0 _charactermovement :!label _label_2)
    (`KismetSystemLibrary.RetriggerableDelay` 0.2)
    (`self.IncreaseStamina`)
    (if (`self.CanIncreaseStamina?`)
      (goto _label_2))))

(event `InputAction|On/Off_Flash`
  (params (Key :type "Key Structure"))
  (bind _spotlight (`self.SpotLight`))
  ;[1 1 1] Flash On/Off
  (:`Pressed`
    (`/Engine/EditorBlueprintResources/StandardMacros.FlipFlop`
      (:`A`
        (if (> (`self.RemainFlashTime`) 0.0)
          (`SceneComponent.SetVisibility` _spotlight true false)
          (set `self.bFlash` true)))
      (:`B`
        (`SceneComponent.SetVisibility` _spotlight false false)
        (set `self.bFlash` false)))))

(event `UseStamina`
  ;[1 1 1] Stamina
  (set `self.stamina` (- (`self.stamina`) 3.0))
  (`GameplayStatics.PlayWorldCameraShake` "/Game/CosmicRestaurant/Blueprints/Adventure/BP_Camerashake.BP_Camerashake_C" (`self.K2_GetActorLocation`) 0.0 1000.0)
  (if (<= (`self.stamina`) 0.0)
    (set `self.bIsRun` false)
    (set `CharacterMovementComponent.MaxWalkSpeed` 600.0 (`self.CharacterMovement`))))

(event `IncreaseStamina`
  ;[1 1 1] Stamina
  (if (<= (`KismetMathLibrary.VSizeXY` (`self.GetVelocity`)) 700.0)
    (set `self.stamina` (+ (`self.stamina`) 1.0))
    (if (>= (`self.stamina`) 100.0)
      (set `self.CanIncreaseStamina?` false)
      (else
        (set `self.CanIncreaseStamina?` true)))))

(fn `UserConstructionScript`)