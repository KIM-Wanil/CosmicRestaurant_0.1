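; First-person player character for Cosmic Restaurant that can sprint on stamina and throw rocks.
; BeginPlay adds the dot HUD and stamina widgets to the viewport.
; IA_Throw plays a montage and spawns BP_ThrowRock at the camera transform.
; Left Shift switches walk speed, with RetriggerableDelay loops draining stamina while sprinting and, after release, refilling it when horizontal speed is low enough.
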(event `self.ReceiveBeginPlay`
  (`|ExecutionSequence`
    (:`then_0`
      (bind _returnvalue (`|CreateWidget` "/Game/Widget/W_DotHud.W_DotHud_C"))
      (`UserWidget.AddToViewport` _returnvalue 0))
    (:`then_1`
      (bind _returnvalue_2 (`|CreateWidget` "/Game/UI/WB_Stamina.WB_Stamina_C" (`GameplayStatics.GetPlayerController` 0)))
      (`UserWidget.AddToViewport` _returnvalue_2 0))))

(event `EnhancedInput|/Game/CosmicRestaurant/Input/Actions/IA_Throw`
  (params (ActionValue :type Boolean) (ElapsedSeconds :type "Float (double-precision)") (TriggeredSeconds :type "Float (double-precision)") (InputAction :type "InputAction Object Reference" :default "/Game/CosmicRestaurant/Input/Actions/IA_Throw.IA_Throw"))
  (bind (_returnvalue_location _returnvalue_rotation) (`KismetMathLibrary.BreakTransform` (`SceneComponent.K2_GetComponentToWorld` (`self.FirstPersonCameraComponent`))))
  (:`Triggered`
    (`|PlayMontage` (`self.Mesh`) "/Game/UsedAssets/CommonResource/FirstPersonArms/Animations/FP_Rifle_Shoot_Montage.FP_Rifle_Shoot_Montage"
      (:`then`
        (`|SpawnActorFromClass` "/Game/CosmicRestaurant/Blueprints/Adventure/Hunting/BP_ThrowRock.BP_ThrowRock_C" (`KismetMathLibrary.MakeTransform` _returnvalue_location _returnvalue_rotation) "AdjustIfPossibleButAlwaysSpawn" "MultiplyWithRoot" null null)))))

(event `Key|LeftShift`
  (params (Key :type "Key Structure"))
  (bind _charactermovement (`self.CharacterMovement`))
  (:`Pressed`
    (set `self.IsRunning?` true)
    (set `CharacterMovementComponent.MaxWalkSpeed` 900.0 _charactermovement :!label _label)
    (`KismetSystemLibrary.RetriggerableDelay` 0.2)
    (`self.UseStamina`)
    (if (`self.IsRunning?`)
      (goto _label)))
  (:`Released`
    (set `self.IsRunning?` false)
    (set `CharacterMovementComponent.MaxWalkSpeed` 600.0 _charactermovement :!label _label_2)
    (`KismetSystemLibrary.RetriggerableDelay` 0.2)
    (`self.IncreaseStamina`)
    (if (`self.CanIncreaseStamina?`)
      (goto _label_2))))

(event `UseStamina`
  (set `self.stamina` (- (`self.stamina`) 1.0))
  (if (<= (`self.stamina`) 0.0)
    (set `self.IsRunning?` false)
    (set `CharacterMovementComponent.MaxWalkSpeed` 600.0 (`self.CharacterMovement`))))

(event `IncreaseStamina`
  (if (<= (`KismetMathLibrary.VSizeXY` (`self.GetVelocity`)) 700.0)
    (set `self.stamina` (+ (`self.stamina`) 2.0))
    (if (>= (`self.stamina`) 100.0)
      (set `self.CanIncreaseStamina?` false)
      (else
        (set `self.CanIncreaseStamina?` true)))))

(fn `UserConstructionScript`)