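; BP_CRCookingCharacter is a first-person cooking character that picks up and carries objects with the left mouse button.
; A camera-forward line trace on press grabs the hit component through a Physics Handle, which Tick holds in front of the camera until release.
; BeginPlay enables the interaction trace component's tick for the locally controlled player and adds a dot HUD widget.
; Collision toggling for held objects is present but unconnected.
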(event `Key|LeftMouseButton`
  (params (Key :type "Key Structure"))
  (bind _firstpersoncameracomponent (`self.FirstPersonCameraComponent`))
  (bind _returnvalue (`SceneComponent.K2_GetComponentLocation` _firstpersoncameracomponent))
  ;[1 1 1] 좌클릭시 잡기
  (:`Pressed`
    (bind (_outhit _returnvalue_2) (`KismetSystemLibrary.LineTraceSingle` :`Start` _returnvalue :`End` (+ _returnvalue (* (`SceneComponent.GetForwardVector` _firstpersoncameracomponent) 500.0)) :`TraceChannel` "TraceTypeQuery4" :`DrawDebugType` "ForDuration"))
    (if _returnvalue_2
      (bind (_bblockinghit _binitialoverlap _time _distance _location _impactpoint _normal _impactnormal _physmat _hitactor _hitcomponent) (`GameplayStatics.BreakHitResult` _outhit))
      (`PhysicsHandleComponent.GrabComponentAtLocationWithRotation` :`self` (`self.PhysicsHandle`) :`Component` _hitcomponent :`Location` (`SceneComponent.K2_GetComponentLocation` _hitcomponent))
      (set `self.Is Carrying` true)))
  (:`Released`
    (if (`self.Is Carrying`)
      (`PhysicsHandleComponent.ReleaseComponent` (`self.PhysicsHandle`))
      (set `self.Is Carrying` false))))

(event `self.ReceiveTick`
  (params (DeltaSeconds :type "Float (single-precision)"))
  (bind _firstpersoncameracomponent (`self.FirstPersonCameraComponent`))
  ;[1 1 1] Object picked UpLoop
  (if (`self.Is Carrying`)
    (`PhysicsHandleComponent.SetTargetLocation` (`self.PhysicsHandle`) (+ (`SceneComponent.K2_GetComponentLocation` _firstpersoncameracomponent) (* (`SceneComponent.GetForwardVector` _firstpersoncameracomponent) 180.0)))))

(event `self.ReceiveBeginPlay`
  ;[1 1 1] 매틱마다 오브젝트를 보고있느지 확인
  (`self.SetupInteractionTrace`)
  (bind _returnvalue (`|CreateWidget` "/Game/Widget/W_DotHud.W_DotHud_C"))
  (`UserWidget.AddToViewport` _returnvalue 0))

(fn `SetupInteractionTrace`
  (if (`self.IsLocallyControlled`)
    (`ActorComponent.SetComponentTickEnabled` (`self.AC_InteractionTrace`) true)))

(fn `UserConstructionScript`)