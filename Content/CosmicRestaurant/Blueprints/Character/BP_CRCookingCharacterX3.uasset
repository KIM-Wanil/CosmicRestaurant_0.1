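; First-person cooking character for Cosmic Restaurant that picks up, carries and drops objects and shows a recipe screen.
; F line-traces from the camera and grabs the hit component with a Physics Handle, which Tick holds in front of the camera until F releases it.
; BeginPlay enables the interaction-trace component for the locally controlled player and creates a dot HUD and a recipe widget, shown while T is held.
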(event `Key|Q`
  (params (Key :type "Key Structure"))
  (:`Pressed`
    (`KismetSystemLibrary.PrintText` "멈춰!")))

(event `Key|F`
  (params (Key :type "Key Structure"))
  (bind _firstpersoncameracomponent (`self.FirstPersonCameraComponent`))
  (bind _returnvalue (`SceneComponent.K2_GetComponentLocation` _firstpersoncameracomponent))
  ;[1 1 1] F로 잡기
  (:`Pressed`
    (if (`self.Is Carrying`)
      (`PhysicsHandleComponent.ReleaseComponent` (`self.PhysicsHandle`))
      (set `self.Is Carrying` false)
      (`self.ReleaseCarrying` (`self.Carrying`))
      (set `self.Carrying` null)
      (else
        (bind (_outhit _returnvalue_2) (`KismetSystemLibrary.LineTraceSingle` :`Start` _returnvalue :`End` (+ _returnvalue (* (`SceneComponent.GetForwardVector` _firstpersoncameracomponent) 500.0)) :`TraceChannel` "TraceTypeQuery3" :`DrawDebugType` "ForDuration"))
        (if _returnvalue_2
          (bind (_bblockinghit _binitialoverlap _time _distance _location _impactpoint _normal _impactnormal _physmat _hitactor _hitcomponent) (`GameplayStatics.BreakHitResult` _outhit))
          (`PhysicsHandleComponent.GrabComponentAtLocationWithRotation` :`self` (`self.PhysicsHandle`) :`Component` _hitcomponent :`Location` (`SceneComponent.K2_GetComponentLocation` _hitcomponent))
          (set `self.Is Carrying` true)
          (set `self.Carrying` _hitactor))))))

(event `self.ReceiveTick`
  (params (DeltaSeconds :type "Float (single-precision)"))
  (bind _firstpersoncameracomponent (`self.FirstPersonCameraComponent`))
  ;[1 1 1] Object picked UpLoop
  (if (`self.Is Carrying`)
    (`PhysicsHandleComponent.SetTargetLocation` (`self.PhysicsHandle`) (+ (`SceneComponent.K2_GetComponentLocation` _firstpersoncameracomponent) (* (`SceneComponent.GetForwardVector` _firstpersoncameracomponent) 180.0)))))

(event `self.ReceiveBeginPlay`
  ;[1 1 1] 매틱마다 오브젝트를 보고있는지 확인
  (`self.SetupInteractionTrace`)
  (bind _returnvalue (`|CreateWidget` "/Game/Widget/W_DotHud.W_DotHud_C"))
  (`UserWidget.AddToViewport` _returnvalue 0)
  (bind _returnvalue_2 (`|CreateWidget` "/Game/CosmicRestaurant/Blueprints/Cooking/RecipeWidget/W_RecipeUI.W_RecipeUI_C"))
  (set `self.RecipeUI` _returnvalue_2)
  (`UserWidget.AddToViewport` _returnvalue_2 0)
  (`Widget.SetVisibility` _returnvalue_2 "Collapsed"))

(event `Key|T`
  (params (Key :type "Key Structure"))
  (bind _recipeui (`self.RecipeUI`))
  (:`Pressed`
    (`Widget.SetVisibility` _recipeui "Visible"))
  (:`Released`
    (`Widget.SetVisibility` _recipeui "Collapsed")))

(fn `SetupInteractionTrace`
  (if (`self.IsLocallyControlled`)
    (`ActorComponent.SetComponentTickEnabled` (`self.AC_InteractionTrace`) true)))

(fn `UserConstructionScript`)