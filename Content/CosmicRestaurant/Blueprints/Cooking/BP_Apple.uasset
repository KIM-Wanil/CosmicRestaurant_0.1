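; BP_Apple is the apple ingredient item for the cooking system.
; Its construction script assigns the apple item data asset and sets the static mesh to that asset's raw-item mesh.
; Interface focus events toggle custom depth rendering on the mesh.
; Cooked and processed state changes defer entirely to the parent class, and the interaction widget getter is an empty stub.
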(event `self.ReceiveBeginPlay`
  (`parent.ReceiveBeginPlay`))

(event `/Game/Interaction/BI_Interaction.Interface_ToggleFocus`
  (params (Focus :type Boolean))
  (`PrimitiveComponent.SetRenderCustomDepth` (`self.StaticMesh`) Focus))

(fn `ChangeToCooked`
  (`parent.ChangeToCooked`))

(fn `ChangeToProcessed`
  (`parent.ChangeToProcessed`))

(fn `GetInteractionWidgetRef`
  (returns (Ref :type "WidgetComponent Object Reference"))
  (return null))

(fn `UserConstructionScript`
  (`parent.UserConstructionScript`)
  (bind _output_get (set `self.ItemData` "/Game/CosmicRestaurant/Data/DA_CookingAppleItem.DA_CookingAppleItem"))
  (`StaticMeshComponent.SetStaticMesh` (`self.StaticMesh`) (`|ConvertAsset` (`CRAdventureItemData.CookingRawItemMesh` _output_get))))