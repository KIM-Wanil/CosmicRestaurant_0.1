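; BP_AppleSpawner is a cooking-station actor that lets the player spawn a BP_Apple by pressing E while in range.
; A sphere overlap shows a prompt widget, sets an Overlapped flag and enables input for player controller 0, without filtering the overlapping actor.
; Leaving hides the widget and clears the flag, which gates the key press because input stays enabled.
; Each press spawns an apple at the spawner's own transform.
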(event `Key|E`
  (params (Key :type "Key Structure"))
  (:`Pressed`
    (if (`self.bOverlapped`)
      (`|SpawnActorFromClass` "/Game/CosmicRestaurant/Blueprints/Cooking/BP_Apple.BP_Apple_C" (`self.GetTransform`) "Undefined" "MultiplyWithRoot" null null))))

(event `self.Sphere.OnComponentBeginOverlap`
  (params (OverlappedComponent :type "PrimitiveComponent Object Reference") (OtherActor :type "Actor Object Reference") (OtherComp :type "PrimitiveComponent Object Reference") (OtherBodyIndex :type Integer) (bFromSweep :type Boolean) (SweepResult :type "HitResult Structure (by ref)"))
  (`SceneComponent.SetVisibility` (`self.Widget`) true false)
  (set `self.bOverlapped` true)
  (`self.EnableInput` (`GameplayStatics.GetPlayerController` 0)))

(event `self.Sphere.OnComponentEndOverlap`
  (params (OverlappedComponent :type "PrimitiveComponent Object Reference") (OtherActor :type "Actor Object Reference") (OtherComp :type "PrimitiveComponent Object Reference") (OtherBodyIndex :type Integer))
  (`SceneComponent.SetVisibility` (`self.Widget`) false false)
  (set `self.bOverlapped` false))

(fn `UserConstructionScript`)