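; Bread ingredient Blueprint for the restaurant cooking system, built on a parent class that handles chopped and processed state changes.
; The construction script assigns the bread data asset and applies its raw mesh, then BeginPlay overrides it with a hardcoded loaf mesh.
; Interaction focus toggles the mesh's custom depth rendering.
; The chop and process overrides only call the parent, and the interaction widget getter returns nothing.
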(event `self.ReceiveBeginPlay`
  (`parent.ReceiveBeginPlay`)
  (`StaticMeshComponent.SetStaticMesh` (`self.StaticMesh`) "/Game/UsedAssets/Food_Pack_01/Meshes/Food_Bread_Loaf_Multi_01.Food_Bread_Loaf_Multi_01"))

(event `/Game/Interaction/BI_Interaction.Interface_ToggleFocus`
  (params (Focus :type Boolean))
  (`PrimitiveComponent.SetRenderCustomDepth` (`self.StaticMesh`) Focus))

(fn `ChangeToChopped`
  (`parent.ChangeToChopped`))

(fn `ChangeToProcessed`
  (params (InputProcessType :type "/Game/CosmicRestaurant/Blueprints/Cooking/EIngredientStatus Enum" :default "NewEnumerator0"))
  (`parent.ChangeToProcessed` InputProcessType))

(fn `GetInteractionWidgetRef`
  (returns (Ref :type "WidgetComponent Object Reference"))
  (return null))

(fn `UserConstructionScript`
  (`parent.UserConstructionScript`)
  (bind _output_get (set `self.ItemData` "/Game/CosmicRestaurant/Data/DA_CookingBreadItem.DA_CookingBreadItem"))
  (`StaticMeshComponent.SetStaticMesh` (`self.StaticMesh`) (`|ConvertAsset` (`CRAdventureItemData.CookingRawItemMesh` _output_get))))