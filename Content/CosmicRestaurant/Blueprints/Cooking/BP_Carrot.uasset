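; BP_Carrot is the carrot ingredient for cooking, a child Blueprint that leaves processing and chopping to its parent.
; Construction assigns the carrot data asset and applies its raw mesh, while BeginPlay sets a hard-coded carrot mesh.
; Focus toggles the mesh's custom depth rendering, and the interaction widget getter returns nothing.
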(event `self.ReceiveBeginPlay`
  (`parent.ReceiveBeginPlay`)
  (`StaticMeshComponent.SetStaticMesh` (`self.StaticMesh`) "/Game/UsedAssets/Food_Pack_01/Meshes/Food_Veg_Carrot_02.Food_Veg_Carrot_02"))

(event `/Game/Interaction/BI_Interaction.Interface_ToggleFocus`
  (params (Focus :type Boolean))
  (`PrimitiveComponent.SetRenderCustomDepth` (`self.StaticMesh`) Focus))

(fn `ChangeToChopped`
  (`parent.ChangeToChopped`))

(fn `ChangeToProcessed`
  (params (InputProcessType :type "/Game/CosmicRestaurant/Blueprints/Cooking/EIngredientStatus Enum" :default "NewEnumerator0"))
  (`parent.ChangeToProcessed` InputProcessType))

(fn `GetInteractionWidgetRef`
  (returns (Ref :type "WidgetComponent Object Reference"))
  (return null))

(fn `UserConstructionScript`
  (`parent.UserConstructionScript`)
  (bind _output_get (set `self.ItemData` "/Game/CosmicRestaurant/Data/DA_CookingCarrotItem.DA_CookingCarrotItem"))
  (`StaticMeshComponent.SetStaticMesh` (`self.StaticMesh`) (`|ConvertAsset` (`CRAdventureItemData.CookingRawItemMesh` _output_get))))