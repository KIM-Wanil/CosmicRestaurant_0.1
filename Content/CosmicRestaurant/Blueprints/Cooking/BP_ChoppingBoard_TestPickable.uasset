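; Test chopping board for a cooking game that holds one carried pickable and lets the nearby player process ingredients on it.
; A person-collider overlap shows the prompt widget, enables input and binds to the cooking character's carry release.
; A released pickable snaps just above the Box and fills the slot until it leaves the Box.
; The CuttingKeyE axis changes a slotted BP_Ingredient's status when it is in either of two eligible states.
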(event `self.ReceiveBeginPlay`
  (bind _asbp_crcooking_character (cast `/Game/CosmicRestaurant/Blueprints/Character/BP_CRCookingCharacter` (`GameplayStatics.GetPlayerCharacter` 0)))
  (set `self.As BP CRCooking Character` _asbp_crcooking_character))

(event `self.Box.OnComponentEndOverlap`
  (params (OverlappedComponent :type "PrimitiveComponent Object Reference") (OtherActor :type "Actor Object Reference") (OtherComp :type "PrimitiveComponent Object Reference") (OtherBodyIndex :type Integer))
  ;[1 1 1] 슬롯비우기
  (set `self.isOverlapped` false)
  (if (== OtherActor (`self.Slot`))
    (set `self.Slot` null)))

(event `InputAxis|CuttingKeyE`
  (params (AxisValue :type "Float (single-precision)"))
  ;[1 1 1] E키 상호작용(최근버전)
  (if (and (`self.isOverlapped`) (`self.isPerson`))
    (if (> AxisValue 0.0)
      (if (`KismetMathLibrary.ClassIsChildOf` (`GameplayStatics.GetObjectClass` (`self.Slot`)) "/Game/CosmicRestaurant/Blueprints/Cooking/BP_Ingredient.BP_Ingredient_C")
        (bind _asbp_ingredient (cast `/Game/CosmicRestaurant/Blueprints/Cooking/BP_Ingredient` (`self.Slot`)))
        (bind _ingredientstatus (`/Game/CosmicRestaurant/Blueprints/Cooking/BP_Ingredient.IngredientStatus` _asbp_ingredient))
        (if (or (`|EnumEquality` _ingredientstatus "NewEnumerator0") (`|EnumEquality` _ingredientstatus "NewEnumerator1"))
          (`/Game/CosmicRestaurant/Blueprints/Cooking/BP_Ingredient.ChangeToProcessed` _asbp_ingredient "NewEnumerator3"))))))

(event `self.personCollider.OnComponentBeginOverlap`
  (params (OverlappedComponent :type "PrimitiveComponent Object Reference") (OtherActor :type "Actor Object Reference") (OtherComp :type "PrimitiveComponent Object Reference") (OtherBodyIndex :type Integer) (bFromSweep :type Boolean) (SweepResult :type "HitResult Structure (by ref)"))
  ;[1 1 1] 인터렉션 UI
  (`SceneComponent.SetVisibility` (`self.Widget`) true false)
  (set `self.isPerson` true)
  (`self.EnableInput` (`GameplayStatics.GetPlayerController` 0))
  (add `/Game/CosmicRestaurant/Blueprints/Character/BP_CRCookingCharacter.ReleaseCarrying` (`self.As BP CRCooking Character`) (delegate `Put`)))

(event `Put`
  (params (Carrying :type "Actor Object Reference"))
  ;[1 1 1] 인터렉션 UI
  (if (not (`self.isOverlapped`))
    (`self.Oning` Carrying)))

(event `self.personCollider.OnComponentEndOverlap`
  (params (OverlappedComponent :type "PrimitiveComponent Object Reference") (OtherActor :type "Actor Object Reference") (OtherComp :type "PrimitiveComponent Object Reference") (OtherBodyIndex :type Integer))
  ;[1 1 1] 인터렉션 UI
  (`SceneComponent.SetVisibility` (`self.Widget`) false false)
  (set `self.isPerson` false))

(event `Oning`
  (params (Carrying :type "Actor Object Reference"))
  (bind (_returnvalue_x _returnvalue_y _returnvalue_z) (`KismetMathLibrary.BreakVector` (`SceneComponent.K2_GetComponentLocation` (`self.Box`))))
  (bind _asbp_pickable (cast `/Game/CosmicRestaurant/Blueprints/Cooking/BP_Pickable` Carrying))
  (`/Engine/EditorBlueprintResources/StandardMacros.IsValid` Carrying
    (:`Is Valid`
      (if (`self.isPerson`)
        (`PrimitiveComponent.SetPhysicsLinearVelocity` (`/Game/CosmicRestaurant/Blueprints/Cooking/BP_Pickable.StaticMesh` _asbp_pickable) (0.0 0.0 0.0) false "None")
        (`self.K2_SetActorLocation` Carrying (`KismetMathLibrary.MakeVector` _returnvalue_x _returnvalue_y (+ _returnvalue_z 10.0)) false false)
        (set `self.isOverlapped` true)
        (set `self.Slot` _asbp_pickable)))))

(fn `UserConstructionScript`)