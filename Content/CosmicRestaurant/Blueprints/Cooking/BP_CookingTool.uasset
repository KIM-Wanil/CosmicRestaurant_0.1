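; BP_CookingTool is a cooking tool actor that holds one ingredient released by the player's cooking character.
; Overlapping SlotCollision enables input and binds Put to the character's ReleaseCarrying event.
; While overlapped and empty, Put accepts a BP_Ingredient, stops its physics, moves it to FoodSlot and snap-attaches it to the tool.
; When that ingredient leaves the collision, its physics resumes and the slot clears.
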(event `self.ReceiveBeginPlay`
  (`parent.ReceiveBeginPlay`)
  (bind _asbp_crcooking_character (cast `/Game/CosmicRestaurant/Blueprints/Character/BP_CRCookingCharacter` (`GameplayStatics.GetPlayerCharacter` 0)))
  (set `self.AsBPCRCookingCharacter` _asbp_crcooking_character))

(event `self.SlotCollision.OnComponentBeginOverlap`
  (params (OverlappedComponent :type "PrimitiveComponent Object Reference") (OtherActor :type "Actor Object Reference") (OtherComp :type "PrimitiveComponent Object Reference") (OtherBodyIndex :type Integer) (bFromSweep :type Boolean) (SweepResult :type "HitResult Structure (by ref)"))
  (set `self.bIsOverlap` true)
  (`self.EnableInput` (`GameplayStatics.GetPlayerController` 0))
  (add `/Game/CosmicRestaurant/Blueprints/Character/BP_CRCookingCharacter.ReleaseCarrying` (`self.AsBPCRCookingCharacter`) (delegate `put`)))

(event `put`
  (params (Carrying :type "Actor Object Reference"))
  (bind _slot (`self.Slot`))
  (bind (_returnvalue_x _returnvalue_y _returnvalue_z) (`KismetMathLibrary.BreakVector` (`SceneComponent.K2_GetComponentLocation` (`self.foodSlot`))))
  (if (`self.bIsOverlap`)
    (if (`self.bIsSlotValid`)
      _
      (elif (`KismetMathLibrary.ClassIsChildOf` (`GameplayStatics.GetObjectClass` Carrying) "/Game/CosmicRestaurant/Blueprints/Cooking/BP_Ingredient.BP_Ingredient_C")
        (bind _asbp_ingredient (cast `/Game/CosmicRestaurant/Blueprints/Cooking/BP_Ingredient` Carrying))
        (set `self.Slot` _asbp_ingredient)
        (set `self.bIsSlotValid` true)
        (`PrimitiveComponent.SetPhysicsLinearVelocity` (`/Game/CosmicRestaurant/Blueprints/Cooking/BP_Pickable.StaticMesh` _asbp_ingredient) (0.0 0.0 0.0) false "None")
        (`self.K2_SetActorLocation` _slot (`KismetMathLibrary.MakeVector` _returnvalue_x _returnvalue_y (+ _returnvalue_z 10.0)) false false)
        (`self.K2_AttachToActor` _slot self "None" "SnapToTarget" "SnapToTarget" "KeepWorld" true)
        (`PrimitiveComponent.SetSimulatePhysics` (`/Game/CosmicRestaurant/Blueprints/Cooking/BP_Pickable.StaticMesh` _slot) false)))))

(event `self.SlotCollision.OnComponentEndOverlap`
  (params (OverlappedComponent :type "PrimitiveComponent Object Reference") (OtherActor :type "Actor Object Reference") (OtherComp :type "PrimitiveComponent Object Reference") (OtherBodyIndex :type Integer))
  (bind _slot (`self.Slot`))
  (set `self.bIsOverlap` false)
  (if (== OtherActor _slot)
    (`PrimitiveComponent.SetSimulatePhysics` (`/Game/CosmicRestaurant/Blueprints/Cooking/BP_Pickable.StaticMesh` _slot) true)
    (set `self.Slot` null)
    (set `self.bIsSlotValid` false)))

(event `Key|Z`
  (params (Key :type "Key Structure"))
  (:`Pressed`
    (`KismetSystemLibrary.PrintText` "Hello")))

(fn `UserConstructionScript`
  (`parent.UserConstructionScript`))