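; BP_Dish is a dish in the restaurant's cooking system that displays the result of a recipe.
; Its SetMesh event stores the recipe info and status/type correctness flags, then picks a mesh.
; An empty recipe name puts a rock mesh on the Rock component; otherwise FoodMesh shows the recipe or incorrect mesh by status.
; IsFood stores the mesh setter's return value in every branch, and TypeCorrect does not affect the mesh.
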(event Custom|SetMesh
  (params (Food :type S%20Recipe%20Row%20Structure) (StatusCorrect :type Boolean) (TypeCorrect :type Boolean))
  (bind (_recipe_name _recipe_mesh _incorrect_mesh) (Utilities|Struct|BreakS_RecipeRow Food))
  (Variables|Default|SetType%20Correct TypeCorrect)
  (bind _output_get (Variables|Default|SetStatus%20Correct StatusCorrect))
  (Variables|Default|SetS_RecipeInfo Food)
  (if (== _recipe_name "")
    (bind _returnvalue (Components|StaticMesh|SetStaticMesh (Variables|Default|GetRock) "/Game/PCG_Test/SM_RockScan_01.SM_RockScan_01"))
    (Variables|Default|SetbIsFood _returnvalue)
    (elif _output_get
      (bind _returnvalue_2 (Components|StaticMesh|SetStaticMesh (Variables|Default|GetFoodMesh) _recipe_mesh))
      (Variables|Default|SetbIsFood _returnvalue_2)
      (else
        (bind _returnvalue_3 (Components|StaticMesh|SetStaticMesh (Variables|Default|GetFoodMesh) _incorrect_mesh))
        (Variables|Default|SetbIsFood _returnvalue_3)))))

(fn ConstructionScript)