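; Grill station for the cooking game that processes an ingredient placed on it while switched on.
; A Sphere overlap shows the interaction widget, enables input for the E on/off toggle and binds to the cooking character's carry-release event.
; A released ingredient snaps above the Box if the slot is free and the player is in range.
; Tick converts it to a processed state if its status qualifies, and leaving the Box frees the slot.
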(event `self.ReceiveBeginPlay`
  (bind _asbp_crcooking_character (cast `/Game/CosmicRestaurant/Blueprints/Character/BP_CRCookingCharacter` (`GameplayStatics.GetPlayerCharacter` 0)))
  (set `self.As BP CRCooking Character` _asbp_crcooking_character))

(event `self.Box.OnComponentBeginOverlap`
  (params (OverlappedComponent :type "PrimitiveComponent Object Reference") (OtherActor :type "Actor Object Reference") (OtherComp :type "PrimitiveComponent Object Reference") (OtherBodyIndex :type Integer) (bFromSweep :type Boolean) (SweepResult :type "HitResult Structure (by ref)"))
  ;[1 1 1] 오버랩
)

(event `self.Box.OnComponentEndOverlap`
  (params (OverlappedComponent :type "PrimitiveComponent Object Reference") (OtherActor :type "Actor Object Reference") (OtherComp :type "PrimitiveComponent Object Reference") (OtherBodyIndex :type Integer))
  ;[1 1 1] 오버랩
  (set `self.isOverlapped` false)
  (if (== OtherActor (`self.CurrIngredient`))
    (set `self.CurrIngredient` null)))

(event `Key|E`
  (params (Key :type "Key Structure"))
  (:`Pressed`
    (if (`self.isPerson`)
      (if (`self.isTurnOn`)
        (set `self.isTurnOn` false)
        (`KismetSystemLibrary.PrintText` "Grill 꺼짐")
        (else
          (set `self.isTurnOn` true)
          (`KismetSystemLibrary.PrintText` "Grill 켜짐" true true (struct :`R` 1.0 :`G` 0.029887 :`A` 1.0)))))))

(event `self.ReceiveTick`
  (params (DeltaSeconds :type "Float (single-precision)"))
  (bind _ingredientstatus (`/Game/CosmicRestaurant/Blueprints/Cooking/BP_Ingredient.IngredientStatus` (`self.CurrIngredient`)))
  (if (and (`self.isTurnOn`) (`self.isOverlapped`))
    (if (or (`|EnumEquality` _ingredientstatus "NewEnumerator0") (`|EnumEquality` _ingredientstatus "NewEnumerator1"))
      (`/Game/CosmicRestaurant/Blueprints/Cooking/BP_Ingredient.ChangeToProcessed` (`self.CurrIngredient`) "NewEnumerator5"))))

(event `self.Sphere.OnComponentBeginOverlap`
  (params (OverlappedComponent :type "PrimitiveComponent Object Reference") (OtherActor :type "Actor Object Reference") (OtherComp :type "PrimitiveComponent Object Reference") (OtherBodyIndex :type Integer) (bFromSweep :type Boolean) (SweepResult :type "HitResult Structure (by ref)"))
  ;[1 1 1] 인터렉션 UI
  (`SceneComponent.SetVisibility` (`self.Widget`) true false)
  (set `self.isPerson` true)
  (`self.EnableInput` (`GameplayStatics.GetPlayerController` 0))
  (add `/Game/CosmicRestaurant/Blueprints/Character/BP_CRCookingCharacter.ReleaseCarrying` (`self.As BP CRCooking Character`) (delegate `Put`)))

(event `Put`
  (params (Carrying :type "Actor Object Reference"))
  ;[1 1 1] 인터렉션 UI
  (if (not (`self.isOverlapped`))
    (`self.Oning` Carrying)))

(event `self.Sphere.OnComponentEndOverlap`
  (params (OverlappedComponent :type "PrimitiveComponent Object Reference") (OtherActor :type "Actor Object Reference") (OtherComp :type "PrimitiveComponent Object Reference") (OtherBodyIndex :type Integer))
  ;[1 1 1] 인터렉션 UI
  (`SceneComponent.SetVisibility` (`self.Widget`) false false)
  (set `self.isPerson` false))

(event `Oning`
  (params (Carrying :type "Actor Object Reference"))
  (bind (_returnvalue_x _returnvalue_y _returnvalue_z) (`KismetMathLibrary.BreakVector` (`SceneComponent.K2_GetComponentLocation` (`self.Box`))))
  (bind _asbp_ingredient (cast `/Game/CosmicRestaurant/Blueprints/Cooking/BP_Ingredient` Carrying))
  (`/Engine/EditorBlueprintResources/StandardMacros.IsValid` Carrying
    (:`Is Valid`
      (if (`self.isPerson`)
        (`PrimitiveComponent.SetPhysicsLinearVelocity` (`/Game/CosmicRestaurant/Blueprints/Cooking/BP_Ingredient.StaticMesh` _asbp_ingredient) (0.0 0.0 0.0) false "None")
        (`self.K2_SetActorLocation` Carrying (`KismetMathLibrary.MakeVector` _returnvalue_x _returnvalue_y (+ _returnvalue_z 10.0)) false false)
        (set `self.isOverlapped` true)
        (bind _asbp_ingredient_2 (cast `/Game/CosmicRestaurant/Blueprints/Cooking/BP_Ingredient` Carrying))
        (set `self.CurrIngredient` _asbp_ingredient_2)))))

(fn `UserConstructionScript`)