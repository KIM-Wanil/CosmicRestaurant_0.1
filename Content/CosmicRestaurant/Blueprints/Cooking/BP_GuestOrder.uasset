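; BP_GuestOrder is a guest order timer for the cooking part of Cosmic Restaurant, pacing how an assigned guest changes posture while waiting.
; SetGuest stores the guest, and Tick accumulates delta time until that guest's time-over flag is set.
; Each time the fixed interval set at BeginPlay elapses, it calls ChangeNextPosture on the guest and restarts the count.
; The attack-player and debug print nodes are disconnected and never run.
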(event `self.ReceiveBeginPlay`
  (set `self.Timer` 5.0)
  (set `self.CurrTimer` 0.0))

(event `self.ReceiveTick`
  (params (DeltaSeconds :type "Float (single-precision)"))
  (if (not (`/Game/CosmicRestaurant/Blueprints/Cooking/Guest/BP_Guest.bIsTImeOver` (`self.Guest`)))
    (`self.CountDownTimer` DeltaSeconds)))

(fn `CountDownTimer`
  (params (DeltaTime :type "Float (double-precision)"))
  (if (>= (`self.CurrTimer`) (`self.Timer`))
    (`/Game/CosmicRestaurant/Blueprints/Cooking/Guest/BP_Guest.ChangeNextPosture` (`self.Guest`))
    (set `self.CurrTimer` 0.0)
    (else
      (set `self.CurrTimer` (+ DeltaTime (`self.CurrTimer`))))))

(fn `SetGuest`
  (params (NewParam :type "/Game/CosmicRestaurant/Blueprints/Cooking/Guest/BP_Guest Object Reference"))
  (set `self.Guest` NewParam))

(fn `UserConstructionScript`)