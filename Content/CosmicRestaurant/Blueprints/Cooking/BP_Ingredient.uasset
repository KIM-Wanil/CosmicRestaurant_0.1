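; BP_Ingredient is an ingredient Blueprint for the cooking system, tracking a status and processing progress.
; BeginPlay resets the status to its first enum value and zeroes the progress.
; Each ChangeToProcessed call increments CurrProcess, or calls ChangeToCooked once MaxProcess has been reached.
; ChangeToCooked is an empty stub, Tick does nothing, and a debug print of the progress is left unconnected.
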(event `self.ReceiveTick`
  (params (DeltaSeconds :type "Float (single-precision)")))

(event `self.ReceiveBeginPlay`
  (set `self.IngredientStatus` "NewEnumerator0")
  (set `self.CurrProcess` 0.0))

(fn `ChangeToCooked`)

(fn `ChangeToProcessed`
  (if (>= (`self.CurrProcess`) (`self.MaxProcess`))
    (`self.ChangeToCooked`)
    (else
      (`/Engine/EditorBlueprintResources/StandardMacros.IncrementFloat` (`self.CurrProcess`)))))

(fn `UserConstructionScript`)