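; Cooking pot that takes four ingredients and turns them into a dish for the player.
; While the player is in range, a widget shows and released ingredients, loose or on a cooking tool, fill the food sockets.
; The fourth triggers an order-independent match against DT_Recipe, checking types and preparation status separately, with status packed as type*10+status.
; Pressing E with an empty BP_Dish transfers the result and clears the pot's meshes.
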(event `self.ReceiveBeginPlay`
  (bind _asbp_crcooking_character (cast `/Game/CosmicRestaurant/Blueprints/Character/BP_CRCookingCharacter` (`GameplayStatics.GetPlayerCharacter` 0)))
  (set `self.As BP CRCooking Character` _asbp_crcooking_character))

(event `self.Sphere.OnComponentBeginOverlap`
  (params (OverlappedComponent :type "PrimitiveComponent Object Reference") (OtherActor :type "Actor Object Reference") (OtherComp :type "PrimitiveComponent Object Reference") (OtherBodyIndex :type Integer) (bFromSweep :type Boolean) (SweepResult :type "HitResult Structure (by ref)"))
  ;[1 1 1] 인터렉션 UI
  (`SceneComponent.SetVisibility` (`self.Widget`) true false)
  (set `self.isPerson` true)
  (`self.EnableInput` (`GameplayStatics.GetPlayerController` 0))
  (add `/Game/CosmicRestaurant/Blueprints/Character/BP_CRCookingCharacter.ReleaseCarrying` (`self.As BP CRCooking Character`) (delegate `Put`))
  (set `self.FoodSocket` (`|MakeArray` (`self.Food0`) (`self.Food1`) (`self.Food2`) (`self.Food3`))))

(event `Put`
  (params (Carrying :type "Actor Object Reference"))
  ;[1 1 1] 인터렉션 UI
  (`self.Oning` Carrying))

(event `self.Sphere.OnComponentEndOverlap`
  (params (OverlappedComponent :type "PrimitiveComponent Object Reference") (OtherActor :type "Actor Object Reference") (OtherComp :type "PrimitiveComponent Object Reference") (OtherBodyIndex :type Integer))
  ;[1 1 1] 인터렉션 UI
  (`SceneComponent.SetVisibility` (`self.Widget`) false false)
  (set `self.isPerson` false))

(event `Oning`
  (params (Carrying :type "Actor Object Reference"))
  (bind _curringredient (`self.CurrIngredient`))
  ;[1 1 1] 솥에 재료 투하
  (if (`self.CanSpawnFood`)
    _
    (elif (`KismetMathLibrary.ClassIsChildOf` (`GameplayStatics.GetObjectClass` Carrying) "/Game/CosmicRestaurant/Blueprints/Cooking/BP_Ingredient.BP_Ingredient_C")
      (bind _asbp_ingredient (cast `/Game/CosmicRestaurant/Blueprints/Cooking/BP_Ingredient` Carrying))
      (bind _output_get (set `self.CurrIngredient` _asbp_ingredient))
      (`/Engine/EditorBlueprintResources/StandardMacros.IsValid` _output_get :!label _label
        (:`Is Valid`
          (if (`self.isPerson`)
            (bind _returnvalue (`KismetArrayLibrary.Array_Add` (`self.IngreTypeDatas`) (`CRAdventureItemData.Type` (`/Game/CosmicRestaurant/Blueprints/Cooking/BP_Ingredient.ItemData` _curringredient))))
            (`KismetArrayLibrary.Array_Add` (`self.IngreStatusDatas`) (`/Game/CosmicRestaurant/Blueprints/Cooking/BP_Ingredient.IngredientStatus` _curringredient))
            (`StaticMeshComponent.SetStaticMesh` (`|GetArrayItem` (`self.FoodSocket`) _returnvalue) (`StaticMeshComponent.StaticMesh` (`/Game/CosmicRestaurant/Blueprints/Cooking/BP_Ingredient.StaticMesh` (`self.CurrIngredient`))))
            (`self.K2_DestroyActor` (`self.CurrIngredient`))
            (if (== _returnvalue 3)
              (set `self.CookedFoodMesh` "/Game/UsedAssets/Adventure/Item/SM_StoneItem.SM_StoneItem")
              (`self.Cook`))))
        (:`Is Not Valid`
          (`KismetSystemLibrary.PrintText` "Hello")))
      (elif (`KismetMathLibrary.ClassIsChildOf` (`GameplayStatics.GetObjectClass` Carrying) "/Game/CosmicRestaurant/Blueprints/Cooking/BP_CookingTool.BP_CookingTool_C")
        (for _array_element (`self.GetAttachedActors` Carrying true false)
          (if (`KismetMathLibrary.ClassIsChildOf` (`GameplayStatics.GetObjectClass` _array_element) "/Game/CosmicRestaurant/Blueprints/Cooking/BP_Ingredient.BP_Ingredient_C")
            (bind _asbp_ingredient_2 (cast `/Game/CosmicRestaurant/Blueprints/Cooking/BP_Ingredient` _array_element))
            (set `self.CurrIngredient` _asbp_ingredient_2)
            (break)))
        (goto _label)))))

(event `Cook`
  ;[1 1 1] 레시피 비교 로직
  (bind _outrownames (`DataTableFunctionLibrary.GetDataTableRowNames` "/Game/CosmicRestaurant/Blueprints/Cooking/DataTable/DT_Recipe.DT_Recipe"))
  (for _array_element _outrownames
    (bind _returnvalue (`|GetDataTableRow` "/Game/CosmicRestaurant/Blueprints/Cooking/DataTable/DT_Recipe.DT_Recipe" _array_element)
      (:`then`
        (bind _output_get (set `self.RecipeStruct` _returnvalue))
        (bind (_exist _statuscorrect) (`self.Compare` (`self.IngreTypeDatas`) (`self.IngreStatusDatas`) (`.1_Type_76_984B542D43E3B12822BE22A0434377A3` (break `/Game/CosmicRestaurant/Blueprints/Cooking/DataTable/S_RecipeRow` _output_get)) (`.2_Type_80_6497623748B7DF3A8786CB9B71BEB505` (break `/Game/CosmicRestaurant/Blueprints/Cooking/DataTable/S_RecipeRow` _output_get)) (`.3_Type_81_A3C94FF9449056F9373EACBA15CE54CD` (break `/Game/CosmicRestaurant/Blueprints/Cooking/DataTable/S_RecipeRow` _output_get)) (`.4_Type_82_10AF7AAF4D312BDA338F2DB720D08B72` (break `/Game/CosmicRestaurant/Blueprints/Cooking/DataTable/S_RecipeRow` _output_get)) (`.1_Status_71_3A125A4443B24CD6FE080C9800777C38` (break `/Game/CosmicRestaurant/Blueprints/Cooking/DataTable/S_RecipeRow` _output_get)) (`.2_Status_83_E1156C654E9CBE167F15CCA234BD2B90` (break `/Game/CosmicRestaurant/Blueprints/Cooking/DataTable/S_RecipeRow` _output_get)) (`.3_Status_84_392601034850132E285EAABEDDF8AA7F` (break `/Game/CosmicRestaurant/Blueprints/Cooking/DataTable/S_RecipeRow` _output_get)) (`.4_Status_85_2150B8274063106DB1541585468E0B6D` (break `/Game/CosmicRestaurant/Blueprints/Cooking/DataTable/S_RecipeRow` _output_get))))
        (bind _output_get_2 (set `self.TypeCorrect` _exist))
        (if _output_get_2
          (set `self.StatusCorrect` _statuscorrect)
          (break)
          (else
            (`KismetSystemLibrary.PrintText` "Faild")
            (set `self.RecipeStruct` (struct)))))))
  (`KismetArrayLibrary.Array_Clear` (`self.IngreTypeDatas`))
  (`KismetArrayLibrary.Array_Clear` (`self.IngreStatusDatas`))
  (set `self.CanSpawnFood` true))

(event `Key|E`
  (params (Key :type "Key Structure"))
  (bind _carrying (`/Game/CosmicRestaurant/Blueprints/Character/BP_CRCookingCharacter.Carrying` (`self.As BP CRCooking Character`)))
  ;[1 1 1] 그릇에 스태틱매시 설정
  (:`Pressed`
    (bind _asbp_dish (cast `/Game/CosmicRestaurant/Blueprints/Cooking/BP_Dish` _carrying))
    (if (and (`self.CanSpawnFood`) (== (`GameplayStatics.GetObjectClass` _carrying) "/Game/CosmicRestaurant/Blueprints/Cooking/BP_Dish.BP_Dish_C") (not (`/Game/CosmicRestaurant/Blueprints/Cooking/BP_Dish.bIsFood` _asbp_dish)))
      (`/Game/CosmicRestaurant/Blueprints/Cooking/BP_Dish.SetMesh` _asbp_dish (`self.RecipeStruct`) (`self.StatusCorrect`) (`self.TypeCorrect`))
      (set `self.CanSpawnFood` false)
      (for _array_element (`self.FoodSocket`)
        (`StaticMeshComponent.SetStaticMesh` _array_element null)))))

(fn `Compare`
  (params (IngreTypeDatas :type "Array of EItemType Enum") (IngreStatusDatas :type "Array of /Game/CosmicRestaurant/Blueprints/Cooking/EIngredientStatus Enum") (`1_Type` :type "EItemType Enum" :default "None") (`2_Type` :type "EItemType Enum" :default "None") (`3_Type` :type "EItemType Enum" :default "None") (`4_Type` :type "EItemType Enum" :default "None") (`1_Status` :type "/Game/CosmicRestaurant/Blueprints/Cooking/EIngredientStatus Enum" :default "NewEnumerator0") (`2_Status` :type "/Game/CosmicRestaurant/Blueprints/Cooking/EIngredientStatus Enum" :default "NewEnumerator0") (`3_Status` :type "/Game/CosmicRestaurant/Blueprints/Cooking/EIngredientStatus Enum" :default "NewEnumerator0") (`4_Status` :type "/Game/CosmicRestaurant/Blueprints/Cooking/EIngredientStatus Enum" :default "NewEnumerator0"))
  (returns (Exist :type Boolean) (StatusCorrect :type Boolean))
  (locals (LocaType :type "Array of EItemType Enum"))
  (bind _output_get (set `local.LocaType` IngreTypeDatas))
  (bind _statuscorrect (`self.Status check` IngreTypeDatas IngreStatusDatas `1_Type` `2_Type` `3_Type` `4_Type` `1_Status` `2_Status` `3_Status` `4_Status`))
  (`|ExecutionSequence`
    (:`then_0`
      (bind _returnvalue (`KismetArrayLibrary.Array_Find` _output_get `1_Type`))
      (bind _output_get_2 (set `self.Exist` (>= _returnvalue 0)))
      (`KismetArrayLibrary.Array_Remove` _output_get _returnvalue))
    (:`then_1`
      (bind _returnvalue_2 (`KismetArrayLibrary.Array_Find` _output_get `2_Type`))
      (bind _output_get_3 (set `self.Exist` (and _output_get_2 (>= _returnvalue_2 0))))
      (`KismetArrayLibrary.Array_Remove` _output_get _returnvalue_2))
    (:`then_2`
      (bind _returnvalue_3 (`KismetArrayLibrary.Array_Find` _output_get `3_Type`))
      (bind _output_get_4 (set `self.Exist` (and _output_get_3 (>= _returnvalue_3 0))))
      (`KismetArrayLibrary.Array_Remove` _output_get _returnvalue_3))
    (:`then_3`
      (bind _returnvalue_4 (`KismetArrayLibrary.Array_Find` _output_get `4_Type`))
      (set `self.Exist` (and _output_get_4 (>= _returnvalue_4 0)))
      (`KismetArrayLibrary.Array_Remove` _output_get _returnvalue_4))
    (:`then_4`
      (return (`self.Exist`) _statuscorrect))))

(fn `Status check`
  (params (IngreTypeDatas :type "Array of EItemType Enum") (IngreStatusDatas :type "Array of /Game/CosmicRestaurant/Blueprints/Cooking/EIngredientStatus Enum") (`1_Type` :type "EItemType Enum" :default "None") (`2_Type` :type "EItemType Enum" :default "None") (`3_Type` :type "EItemType Enum" :default "None") (`4_Type` :type "EItemType Enum" :default "None") (`1_Status` :type "/Game/CosmicRestaurant/Blueprints/Cooking/EIngredientStatus Enum" :default "NewEnumerator0") (`2_Status` :type "/Game/CosmicRestaurant/Blueprints/Cooking/EIngredientStatus Enum" :default "NewEnumerator0") (`3_Status` :type "/Game/CosmicRestaurant/Blueprints/Cooking/EIngredientStatus Enum" :default "NewEnumerator0") (`4_Status` :type "/Game/CosmicRestaurant/Blueprints/Cooking/EIngredientStatus Enum" :default "NewEnumerator0"))
  (returns (StatusCorrect :type Boolean))
  (locals (RecipeNums :type "Array of Integer64"))
  (bind _recipenums (`local.RecipeNums`))
  (bind _recipenums_2 (`local.RecipeNums`))
  (bind _returnvalue (`KismetArrayLibrary.Array_Find` _recipenums (+ (* (`KismetMathLibrary.Conv_ByteToInt64` `1_Type`) 10) (`KismetMathLibrary.Conv_ByteToInt64` `1_Status`))))
  (bind _returnvalue_2 (`KismetArrayLibrary.Array_Find` _recipenums (+ (* (`KismetMathLibrary.Conv_ByteToInt64` `2_Type`) 10) (`KismetMathLibrary.Conv_ByteToInt64` `2_Status`))))
  (bind _returnvalue_3 (`KismetArrayLibrary.Array_Find` _recipenums (+ (* (`KismetMathLibrary.Conv_ByteToInt64` `4_Type`) 10) (`KismetMathLibrary.Conv_ByteToInt64` `4_Status`))))
  (bind _returnvalue_4 (`KismetArrayLibrary.Array_Find` _recipenums (+ (* (`KismetMathLibrary.Conv_ByteToInt64` `3_Type`) 10) (`KismetMathLibrary.Conv_ByteToInt64` `3_Status`))))
  (`|ExecutionSequence`
    (:`then_0`
      (for (_array_element _array_index) IngreTypeDatas
        (`KismetArrayLibrary.Array_Add` (`local.RecipeNums`) (+ (* (`KismetMathLibrary.Conv_ByteToInt64` _array_element) 10) (`KismetMathLibrary.Conv_ByteToInt64` (`|GetArrayItem` IngreStatusDatas _array_index))))))
    (:`then_1`
      (`|ExecutionSequence`
        (:`then_0`
          (bind _output_get (set `self.StatusCheck` (>= _returnvalue 0)))
          (`KismetArrayLibrary.Array_Remove` _recipenums_2 _returnvalue))
        (:`then_1`
          (bind _output_get_2 (set `self.StatusCheck` (and _output_get (>= _returnvalue_2 0))))
          (`KismetArrayLibrary.Array_Remove` _recipenums_2 _returnvalue_2))
        (:`then_2`
          (bind _output_get_3 (set `self.StatusCheck` (and _output_get_2 (>= _returnvalue_4 0))))
          (`KismetArrayLibrary.Array_Remove` _recipenums_2 _returnvalue_4))
        (:`then_3`
          (set `self.StatusCheck` (and _output_get_3 (>= _returnvalue_3 0)))
          (`KismetArrayLibrary.Array_Remove` _recipenums_2 _returnvalue_3))))
    (:`then_2`
      (return (`self.StatusCheck`)))))

(fn `UserConstructionScript`)