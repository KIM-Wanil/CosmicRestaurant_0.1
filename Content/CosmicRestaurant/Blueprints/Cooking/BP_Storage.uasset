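; BP_Storage is a cooking storage actor that opens the WBP_CookStorage screen when E is pressed.
; Sphere overlap shows or hides a widget and sets an Overlapped flag, and entering also enables input, which is never disabled.
; The E handler checks only StorageOpen, which is never reset here, so the screen is created once.
; Unconnected leftover logic prints GI_Inventory's TempInventory and spawns BP_Fruit.
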(event `Key|E`
  (params (Key :type "Key Structure"))
  (:`Pressed`
    (if (not (`self.bStorageOpen`))
      (set `self.bStorageOpen` true)
      (bind _returnvalue (`|CreateWidget` "/Game/CosmicRestaurant/Blueprints/UI/CookPartUI/WBP_CookStorage.WBP_CookStorage_C"))
      (`UserWidget.AddToViewport` _returnvalue 0)
      (`KismetSystemLibrary.Delay` 3.0))))

(event `self.Sphere.OnComponentBeginOverlap`
  (params (OverlappedComponent :type "PrimitiveComponent Object Reference") (OtherActor :type "Actor Object Reference") (OtherComp :type "PrimitiveComponent Object Reference") (OtherBodyIndex :type Integer) (bFromSweep :type Boolean) (SweepResult :type "HitResult Structure (by ref)"))
  (`SceneComponent.SetVisibility` (`self.Widget`) true false)
  (set `self.bOverlapped` true)
  (`self.EnableInput` (`GameplayStatics.GetPlayerController` 0)))

(event `self.Sphere.OnComponentEndOverlap`
  (params (OverlappedComponent :type "PrimitiveComponent Object Reference") (OtherActor :type "Actor Object Reference") (OtherComp :type "PrimitiveComponent Object Reference") (OtherBodyIndex :type Integer))
  (`SceneComponent.SetVisibility` (`self.Widget`) false false)
  (set `self.bOverlapped` false))

(fn `UserConstructionScript`)