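; BP_Stove is a cooking stove the player toggles with E while in range, shown by a fire effect and interaction widget.
; Entering range binds to the cooking character's release-carrying event, which snaps a dropped pickable onto the stove if empty.
; While lit, Tick checks for a cooking tool on top and calls its ingredient's change function according to ingredient status, passing the tool's cook type for raw or processed food.
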(event `self.ReceiveBeginPlay`
  (bind _asbp_crcooking_character (cast `/Game/CosmicRestaurant/Blueprints/Character/BP_CRCookingCharacter` (`GameplayStatics.GetPlayerCharacter` 0)))
  (set `self.As BP CRCooking Character` _asbp_crcooking_character))

(event `self.Box.OnComponentEndOverlap`
  (params (OverlappedComponent :type "PrimitiveComponent Object Reference") (OtherActor :type "Actor Object Reference") (OtherComp :type "PrimitiveComponent Object Reference") (OtherBodyIndex :type Integer))
  ;[1 1 1] 오버랩
  (if (== OtherActor (`self.Slot`))
    (set `self.Slot` null)
    (set `self.isOverlapped` false)))

(event `Key|E`
  (params (Key :type "Key Structure"))
  (bind _fire (`self.fire`))
  ;[1 1 1] E키로 불 켜고 끄기
  (:`Pressed`
    (if (`self.isPerson`)
      (if (`self.isTurnOn`)
        (set `self.isTurnOn` false)
        (`KismetSystemLibrary.PrintText` "CookingPot 꺼짐")
        (`SceneComponent.SetVisibility` _fire false true)
        (else
          (set `self.isTurnOn` true)
          (`KismetSystemLibrary.PrintText` "CookingPot 켜짐" true true (struct :`R` 1.0 :`B` 0.045152 :`A` 1.0))
          (`SceneComponent.SetVisibility` _fire true true))))))

(event `self.PersonCollider.OnComponentBeginOverlap`
  (params (OverlappedComponent :type "PrimitiveComponent Object Reference") (OtherActor :type "Actor Object Reference") (OtherComp :type "PrimitiveComponent Object Reference") (OtherBodyIndex :type Integer) (bFromSweep :type Boolean) (SweepResult :type "HitResult Structure (by ref)"))
  ;[1 1 1] 인터렉션 UI
  (`SceneComponent.SetVisibility` (`self.Widget`) true false)
  (set `self.isPerson` true)
  (`self.EnableInput` (`GameplayStatics.GetPlayerController` 0))
  (add `/Game/CosmicRestaurant/Blueprints/Character/BP_CRCookingCharacter.ReleaseCarrying` (`self.As BP CRCooking Character`) (delegate `Put`)))

(event `Put`
  (params (Carrying :type "Actor Object Reference"))
  ;[1 1 1] 인터렉션 UI
  (if (not (`self.isOverlapped`))
    (`self.Oning` Carrying)))

(event `self.ReceiveTick`
  (params (DeltaSeconds :type "Float (single-precision)"))
  ;[1 1 1] 불이 켜져있고, 위에 음식재료가 있다면 해당 음식재료 process 함수 호출
  (if (and (`self.isTurnOn`) (`self.isOverlapped`))
    (if (`KismetMathLibrary.ClassIsChildOf` (`GameplayStatics.GetObjectClass` (`self.Slot`)) "/Game/CosmicRestaurant/Blueprints/Cooking/BP_CookingTool.BP_CookingTool_C")
      (bind _asbp_cooking_tool (cast `/Game/CosmicRestaurant/Blueprints/Cooking/BP_CookingTool` (`self.Slot`)))
      (if (`/Game/CosmicRestaurant/Blueprints/Cooking/BP_CookingTool.bIsSlotValid` _asbp_cooking_tool)
        (bind _slot (`/Game/CosmicRestaurant/Blueprints/Cooking/BP_CookingTool.Slot` _asbp_cooking_tool))
        (switch `/Game/CosmicRestaurant/Blueprints/Cooking/EIngredientStatus` (`/Game/CosmicRestaurant/Blueprints/Cooking/BP_Ingredient.IngredientStatus` _slot)
          (:`NewEnumerator0`
            (`/Game/CosmicRestaurant/Blueprints/Cooking/BP_Ingredient.ChangeToProcessed` _slot (`/Game/CosmicRestaurant/Blueprints/Cooking/BP_CookingTool.CookType` _asbp_cooking_tool) :!label _label))
          (:`NewEnumerator1`
            (goto _label))
          (:`NewEnumerator4`
            (`/Game/CosmicRestaurant/Blueprints/Cooking/BP_Ingredient.ChangeToBoiled` _slot))
          (:`NewEnumerator5`
            (`/Game/CosmicRestaurant/Blueprints/Cooking/BP_Ingredient.Change to Grilled` _slot)))))))

(event `self.PersonCollider.OnComponentEndOverlap`
  (params (OverlappedComponent :type "PrimitiveComponent Object Reference") (OtherActor :type "Actor Object Reference") (OtherComp :type "PrimitiveComponent Object Reference") (OtherBodyIndex :type Integer))
  ;[1 1 1] 인터렉션 UI
  (`SceneComponent.SetVisibility` (`self.Widget`) false false)
  (set `self.isPerson` false))

(event `Oning`
  (params (Carrying :type "Actor Object Reference"))
  (bind (_returnvalue_x _returnvalue_y _returnvalue_z) (`KismetMathLibrary.BreakVector` (`SceneComponent.K2_GetComponentLocation` (`self.Box`))))
  (bind _asbp_pickable (cast `/Game/CosmicRestaurant/Blueprints/Cooking/BP_Pickable` Carrying))
  (`/Engine/EditorBlueprintResources/StandardMacros.IsValid` Carrying
    (:`Is Valid`
      (if (`self.isPerson`)
        (`PrimitiveComponent.SetPhysicsLinearVelocity` (`/Game/CosmicRestaurant/Blueprints/Cooking/BP_Pickable.StaticMesh` _asbp_pickable) (0.0 0.0 0.0) false "None")
        (`self.K2_SetActorLocation` Carrying (`KismetMathLibrary.MakeVector` _returnvalue_x _returnvalue_y (+ _returnvalue_z 10.0)) false false)
        (set `self.isOverlapped` true)
        (set `self.Slot` _asbp_pickable)))))

(fn `UserConstructionScript`)