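; BP_TrashCan is a trash can for the cooking game that disposes of ingredients the player releases nearby.
; Sphere overlap sets a proximity flag, enables input and binds Throw to the cooking character's ReleaseCarrying event; end overlap only clears the flag.
; While flagged, Throw destroys a released ingredient, or only the first ingredient directly attached to any other released item, leaving that item intact.
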(event `self.ReceiveBeginPlay`
  (bind _asbp_crcooking_character (cast `/Game/CosmicRestaurant/Blueprints/Character/BP_CRCookingCharacter` (`GameplayStatics.GetPlayerCharacter` 0)))
  (set `self.As BP CRCookinCharacter` _asbp_crcooking_character))

(event `self.Sphere.OnComponentBeginOverlap`
  (params (OverlappedComponent :type "PrimitiveComponent Object Reference") (OtherActor :type "Actor Object Reference") (OtherComp :type "PrimitiveComponent Object Reference") (OtherBodyIndex :type Integer) (bFromSweep :type Boolean) (SweepResult :type "HitResult Structure (by ref)"))
  (set `self.bIsPerson` true)
  (`self.EnableInput` (`GameplayStatics.GetPlayerController` 0))
  (add `/Game/CosmicRestaurant/Blueprints/Character/BP_CRCookingCharacter.ReleaseCarrying` (`self.As BP CRCookinCharacter`) (delegate `Throw`)))

(event `Throw`
  (params (Carrying :type "Actor Object Reference"))
  (if (`self.bIsPerson`)
    (if (`KismetMathLibrary.ClassIsChildOf` (`GameplayStatics.GetObjectClass` Carrying) "/Game/CosmicRestaurant/Blueprints/Cooking/BP_Ingredient.BP_Ingredient_C")
      (`self.K2_DestroyActor` Carrying)
      (else
        (for _array_element (`self.GetAttachedActors` Carrying true false)
          (if (`KismetMathLibrary.ClassIsChildOf` (`GameplayStatics.GetObjectClass` _array_element) "/Game/CosmicRestaurant/Blueprints/Cooking/BP_Ingredient.BP_Ingredient_C")
            (`self.K2_DestroyActor` _array_element)
            (break)))))))

(event `self.Sphere.OnComponentEndOverlap`
  (params (OverlappedComponent :type "PrimitiveComponent Object Reference") (OtherActor :type "Actor Object Reference") (OtherComp :type "PrimitiveComponent Object Reference") (OtherBodyIndex :type Integer))
  (set `self.bIsPerson` false))

(fn `UserConstructionScript`)