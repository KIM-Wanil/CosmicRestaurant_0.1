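; Base restaurant guest for the cooking game that takes a random free chair, receives a dish from the player and reacts to it.
; Its MobType, meant to be set by children, selects taste preferences from DT_GuestPreference, while BPOrder is bound to the guest.
; Releasing a carried item inside FoodBox blinks lights, starts a fade-out exit, and reports satisfaction from dish type scores and correctness.
; Chair tags track seat availability.
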(event `self.ReceiveBeginPlay`
  (bind _bp_order (`self.BP_Order`))
  (`/Game/CosmicRestaurant/Blueprints/Cooking/Guest/BP_Order.SetGuest` _bp_order self)
  (`ActorComponent.SetComponentTickEnabled` _bp_order true)
  (bind _asbp_crcooking_character (cast `/Game/CosmicRestaurant/Blueprints/Character/BP_CRCookingCharacter` (`GameplayStatics.GetPlayerCharacter` 0)))
  (set `self.As BP CRCooking Character` _asbp_crcooking_character)
  ;[1 1 1] 자손에서 Type setting
  (`self.SetMobType` (`self.MobType`))
  (`self.MoveToChair`))

(event `self.FoodBox.OnComponentBeginOverlap`
  (params (OverlappedComponent :type "PrimitiveComponent Object Reference") (OtherActor :type "Actor Object Reference") (OtherComp :type "PrimitiveComponent Object Reference") (OtherBodyIndex :type Integer) (bFromSweep :type Boolean) (SweepResult :type "HitResult Structure (by ref)"))
  ;[1 1 1] 음식 제공 상호작용
  (set `self.bIs Person` true)
  (add `/Game/CosmicRestaurant/Blueprints/Character/BP_CRCookingCharacter.ReleaseCarrying` (`self.As BP CRCooking Character`) (delegate `Release`)))

(event `Release`
  (params (Carrying :type "Actor Object Reference"))
  ;[1 1 1] 음식 제공 상호작용
  (if (`self.bIs Person`)
    (`self.GiveFood` Carrying)))

(event `self.FoodBox.OnComponentEndOverlap`
  (params (OverlappedComponent :type "PrimitiveComponent Object Reference") (OtherActor :type "Actor Object Reference") (OtherComp :type "PrimitiveComponent Object Reference") (OtherBodyIndex :type Integer))
  ;[1 1 1] 음식 제공 상호작용
  (set `self.bIs Person` false))

(event `GiveFood`
  (params (Carrying :type "Actor Object Reference"))
  (bind (_monstertype _typescore) (break `/Game/CosmicRestaurant/Blueprints/Cooking/DataTable/S_GuestPreference` (`self.MobPreference`)))
  ;[1 1 1] 음식 비교
  (`self.Blink`)
  (`KismetSystemLibrary.Delay` 2.0)
  (`self.Exit`)
  (bind _asbp_dish (cast `/Game/CosmicRestaurant/Blueprints/Cooking/BP_Dish` Carrying))
  (set `self.As BP Dish` _asbp_dish)
  (bind ((`1_Type_76_984B542D43E3B12822BE22A0434377A3` _1_type) (`2_Type_80_6497623748B7DF3A8786CB9B71BEB505` _2_type) (`3_Type_81_A3C94FF9449056F9373EACBA15CE54CD` _3_type) (`4_Type_82_10AF7AAF4D312BDA338F2DB720D08B72` _4_type)) (break `/Game/CosmicRestaurant/Blueprints/Cooking/DataTable/S_RecipeRow` (`/Game/CosmicRestaurant/Blueprints/Cooking/BP_Dish.S_RecipeInfo` _asbp_dish)))
  (bind _statesatis (`self.SetSatis` (+ (`BlueprintMapLibrary.Map_Find` _typescore _1_type) (`BlueprintMapLibrary.Map_Find` _typescore _2_type) (`BlueprintMapLibrary.Map_Find` _typescore _3_type) (`BlueprintMapLibrary.Map_Find` _typescore _4_type))))
  (if (`/Game/CosmicRestaurant/Blueprints/Cooking/BP_Dish.Type Correct` (`self.As BP Dish`))
    (if (`/Game/CosmicRestaurant/Blueprints/Cooking/BP_Dish.Status Correct` (`self.As BP Dish`))
      (`self.GuestSatisfaction` _statesatis)
      (else
        (`self.GuestSatisfaction` -1)))
    (else
      (`self.GuestSatisfaction` -1)))
  (`/Game/CosmicRestaurant/Blueprints/Cooking/BP_Dish.Reset` (`self.As BP Dish`)))

(event `Exit`
  (bind _returnvalue (`GameplayStatics.GetPlayerCameraManager` 0))
  ;[1 1 1] 손님 퇴장 이펙트
  (`PlayerCameraManager.StartCameraFade` :`self` _returnvalue :`ToAlpha` 1.0 :`Duration` 0.5 :`bHoldWhenFinished` true)
  (`KismetSystemLibrary.Delay` 1.0)
  (`PlayerCameraManager.StartCameraFade` :`self` _returnvalue :`FromAlpha` 1.0 :`Duration` 0.5 :`bHoldWhenFinished` true)
  (`/Game/CosmicRestaurant/Blueprints/Cooking/Guest/BP_Chair.SeatTrue` (`self.Chair`))
  (`self.K2_DestroyActor`))

(event `Blink`
  ;[1 1 1] 불빛 깜박이게
  (bind _outactors (`GameplayStatics.GetAllActorsOfClass` "/Game/CosmicRestaurant/Blueprints/Cooking/Guest/BP_Light.BP_Light_C"))
  (for _array_element _outactors
    (`/Game/CosmicRestaurant/Blueprints/Cooking/Guest/BP_Light.Blink` _array_element)))

(fn `AttackPlayer`
  (`KismetSystemLibrary.PrintText` "GameOver" true true (struct :`R` 1.0 :`G` 0.075957 :`A` 1.0) 10.0))

(fn `ChangeNextPosture`)

(fn `MoveToChair`
  (returns (Sucess :type Boolean) (Chair :type "/Game/CosmicRestaurant/Blueprints/Cooking/Guest/BP_Chair Object Reference"))
  (locals (NewLocalVar :type "/Game/CosmicRestaurant/Blueprints/Cooking/Guest/BP_Chair Object Reference"))
  ;[1 1 1] 랜덤한 의자 설정
  (bind _outactors (`GameplayStatics.GetAllActorsOfClassWithTag` "/Game/CosmicRestaurant/Blueprints/Cooking/Guest/BP_Chair.BP_Chair_C" "True"))
  (bind _output_get (set `self.Chair` (`|GetArrayItem` _outactors (`KismetMathLibrary.RandomInteger` (`KismetArrayLibrary.Array_Length` _outactors)))))
  (`/Engine/EditorBlueprintResources/StandardMacros.IsValid` _output_get
    (:`Is Valid`
      (`AIBlueprintHelperLibrary.SimpleMoveToActor` (`self.GetController`) _output_get)
      (set `Actor.Tags` (`|MakeArray` "False" :!type "Name") _output_get)
      (return true null))
    (:`Is Not Valid`
      (return false _output_get))))

(fn `SetMobType`
  (params (MobType :type "/Game/CosmicRestaurant/Blueprints/Cooking/DataTable/E_MonsterType Enum" :default "NewEnumerator0"))
  (bind _returnvalue (`|GetDataTableRow` "/Game/CosmicRestaurant/Blueprints/Cooking/DataTable/DT_GuestPreference.DT_GuestPreference" (`KismetStringLibrary.Conv_StringToName` (`|GetEnumeratorNameAsString` MobType)))
    (:`then`
      (set `self.MobPreference` _returnvalue))))

(fn `SetSatis`
  (params (Satisfaction :type Integer))
  (returns (StateSatis :type Integer))
  (locals (Satis :type Integer))
  (bind _output_get (set `local.Satis` Satisfaction))
  (if (< _output_get 0)
    (return -1)
    (else
      (return 0))))

(fn `UserConstructionScript`)