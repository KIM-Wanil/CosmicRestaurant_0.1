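; BP_NailGirlGuest is the Nail Girl guest for the cooking part of Cosmic Restaurant, a child of a parent guest Blueprint.
; On BeginPlay it sets its MobType before running the parent logic.
; Each ChangeNextPosture call runs the parent version, increments PostureNum and loops the matching Nail Girl animation on the mesh.
; When the count reaches the last stage, it attacks the player and flags time as over.
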(event `self.ReceiveBeginPlay`
  (set `self.MobType` "NewEnumerator2")
  (`parent.ReceiveBeginPlay`))

(fn `ChangeNextPosture`
  (`parent.ChangeNextPosture`)
  (`/Engine/EditorBlueprintResources/StandardMacros.IncrementInt` (`self.PostureNum`)
    (:`  `
      (switch `int` (`self.PostureNum`)
        (:`0`
          (`SkeletalMeshComponent.PlayAnimation` (`self.Mesh`) "/Game/CosmicRestaurant/Blueprints/Cooking/Guest/GuestAnim/NailGirl/NailGirl_1.NailGirl_1" true))
        (:`1`
          (`SkeletalMeshComponent.PlayAnimation` (`self.Mesh`) "/Game/CosmicRestaurant/Blueprints/Cooking/Guest/GuestAnim/NailGirl/NailGirl_2.NailGirl_2" true))
        (:`2`
          (`SkeletalMeshComponent.PlayAnimation` (`self.Mesh`) "/Game/CosmicRestaurant/Blueprints/Cooking/Guest/GuestAnim/NailGirl/NailGirl_3.NailGirl_3" true))
        (:`3`
          (`self.AttackPlayer`)
          (set `self.bIsTImeOver` true))))))

(fn `UserConstructionScript`
  (`parent.UserConstructionScript`))