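; Twig variant of a restaurant guest that escalates through postures and ends by attacking the player.
; It sets its mob type on BeginPlay before running the parent logic.
; Its ChangeNextPosture override calls the parent, increments the posture counter and plays the matching animation, choosing randomly between two variants at the third stage.
; The final stage triggers AttackPlayer and flags time as over.
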(event `self.ReceiveBeginPlay`
  (`self.SetMobType` "NewEnumerator0")
  (`parent.ReceiveBeginPlay`))

(event `self.ReceiveTick`
  (params (DeltaSeconds :type "Float (single-precision)")))

(fn `ChangeNextPosture`
  (`parent.ChangeNextPosture`)
  (`/Engine/EditorBlueprintResources/StandardMacros.IncrementInt` (`self.PostureNum`)
    (:`  `
      (switch `int` (`self.PostureNum`)
        (:`0`
          (`SkeletalMeshComponent.PlayAnimation` (`self.Mesh`) "/Game/CosmicRestaurant/Blueprints/Cooking/Guest/GuestAnim/Twig/Anim_GuestTwig_Idle.Anim_GuestTwig_Idle" true))
        (:`1`
          (`SkeletalMeshComponent.PlayAnimation` (`self.Mesh`) "/Game/CosmicRestaurant/Blueprints/Cooking/Guest/GuestAnim/Twig/Anim_GuestTwig_2.Anim_GuestTwig_2" true))
        (:`2`
          (if (== (`KismetMathLibrary.RandomInteger` 2) 0)
            (`SkeletalMeshComponent.PlayAnimation` (`self.Mesh`) "/Game/CosmicRestaurant/Blueprints/Cooking/Guest/GuestAnim/Twig/Anim_GuestTwig_2-3.Anim_GuestTwig_2-3" false)
            (else
              (`SkeletalMeshComponent.PlayAnimation` (`self.Mesh`) "/Game/CosmicRestaurant/Blueprints/Cooking/Guest/GuestAnim/Twig/Anim_GuestTwig_2-2.Anim_GuestTwig_2-2" true))))
        (:`3`
          (`self.AttackPlayer`)
          (set `self.bIsTImeOver` true))))))

(fn `UserConstructionScript`
  (`parent.UserConstructionScript`))