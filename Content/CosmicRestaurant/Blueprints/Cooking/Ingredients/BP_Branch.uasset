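; BP_Branch is the branch ingredient actor for cooking, set up from the DA_BranchItem data asset.
; Its construction script runs the parent's, assigns that item data and applies its raw cooking mesh to the static mesh.
; The focus interface event toggles Render Custom Depth on that mesh.
; GetInteractionWidgetRef returns no widget.
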(event `self.Interface_ToggleFocus`
  (params (Focus :type Boolean))
  (`PrimitiveComponent.SetRenderCustomDepth` (`self.StaticMesh`) Focus))

(fn `GetInteractionWidgetRef`
  (returns (Ref :type "WidgetComponent Object Reference"))
  (return null))

(fn `UserConstructionScript`
  (`parent.UserConstructionScript`)
  (bind _output_get (set `self.ItemData` "/Game/CosmicRestaurant/Data/ItemData/DA_BranchItem.DA_BranchItem"))
  (`StaticMeshComponent.SetStaticMesh` (`self.StaticMesh`) (`|ConvertAsset` (`CRAdventureItemData.CookingRawItemMesh` _output_get))))