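; Base restaurant guest for the cooking game that walks to a chair, receives food from the player and leaves.
; On BeginPlay it moves to a random chair tagged "True" and retags it "False" to claim it.
; While its FoodBox is overlapped, a player release of any carried BP_Dish triggers exit, without checking the recipe.
; Exit destroys the guest behind a camera fade; a light-blink alternative is left unconnected.
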(event `self.ReceiveBeginPlay`
  (`self.MoveToChair`)
  (bind _asbp_crcooking_character (cast `/Game/CosmicRestaurant/Blueprints/Character/BP_CRCookingCharacter` (`GameplayStatics.GetPlayerCharacter` 0)))
  (set `self.As BP CRCooking Character` _asbp_crcooking_character))

(event `self.FoodBox.OnComponentBeginOverlap`
  (params (OverlappedComponent :type "PrimitiveComponent Object Reference") (OtherActor :type "Actor Object Reference") (OtherComp :type "PrimitiveComponent Object Reference") (OtherBodyIndex :type Integer) (bFromSweep :type Boolean) (SweepResult :type "HitResult Structure (by ref)"))
  ;[1 1 1] 음식 제공 상호작용
  (set `self.bIs Person` true)
  (add `/Game/CosmicRestaurant/Blueprints/Character/BP_CRCookingCharacter.ReleaseCarrying` (`self.As BP CRCooking Character`) (delegate `Release`)))

(event `Release`
  (params (Carrying :type "Actor Object Reference"))
  ;[1 1 1] 음식 제공 상호작용
  (if (`self.bIs Person`)
    (`self.GiveFood` Carrying)))

(event `self.FoodBox.OnComponentEndOverlap`
  (params (OverlappedComponent :type "PrimitiveComponent Object Reference") (OtherActor :type "Actor Object Reference") (OtherComp :type "PrimitiveComponent Object Reference") (OtherBodyIndex :type Integer))
  ;[1 1 1] 음식 제공 상호작용
  (set `self.bIs Person` false))

(event `GiveFood`
  (params (Carrying :type "Actor Object Reference"))
  (bind _asbp_dish (cast `/Game/CosmicRestaurant/Blueprints/Cooking/BP_Dish` Carrying))
  (`self.Exit`))

(event `Exit`
  (bind _returnvalue (`GameplayStatics.GetPlayerCameraManager` 0))
  ;[1 1 1] 손님 퇴장 이펙트
  (`PlayerCameraManager.StartCameraFade` :`self` _returnvalue :`ToAlpha` 1.0 :`Duration` 0.5 :`bHoldWhenFinished` true)
  (`KismetSystemLibrary.Delay` 1.0)
  (`PlayerCameraManager.StartCameraFade` :`self` _returnvalue :`FromAlpha` 1.0 :`Duration` 0.5 :`bHoldWhenFinished` true)
  ;;[1 1 1] 또는 불빛 깜박이게
  (`self.K2_DestroyActor`))

(fn `MoveToChair`
  (locals (NewLocalVar :type "/Game/CosmicRestaurant/Blueprints/Cooking/Guest/BP_Chair Object Reference"))
  ;[1 1 1] 랜덤한 의자 설정
  (bind _outactors (`GameplayStatics.GetAllActorsOfClassWithTag` "/Game/CosmicRestaurant/Blueprints/Cooking/Guest/BP_Chair.BP_Chair_C" "True"))
  (bind _output_get (set `local.NewLocalVar` (`|GetArrayItem` _outactors (`KismetMathLibrary.RandomInteger` (`KismetArrayLibrary.Array_Length` _outactors)))))
  (`AIBlueprintHelperLibrary.SimpleMoveToActor` (`self.GetController`) _output_get)
  (set `Actor.Tags` (`|MakeArray` "False" :!type "Name") _output_get))

(fn `UserConstructionScript`)