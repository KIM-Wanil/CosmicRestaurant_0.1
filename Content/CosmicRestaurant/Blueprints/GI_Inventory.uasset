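; Game Instance for Cosmic Restaurant that holds a temporary copy of inventory data, sized to 15 slots on Init.
; SaveInventoryData resizes TempInventory to match the passed array and copies it slot by slot.
; LoadInventoryData does the reverse, resizing and filling the passed array from the stored copy.
; DebugData prints each slot's index, item name and quantity.
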(event `self.ReceiveInit`
  (`KismetArrayLibrary.Array_Resize` (`self.TempInventory`) 15))

(fn `DebugData`
  (for (_array_element _array_index) (`self.TempInventory`)
    (bind (_name _quantity) (break `/Game/CosmicRestaurant/Blueprints/UI/Gaeun_Folder/Inventory/Inventory_Wanil/FSlotStructure` _array_element))
    (`KismetSystemLibrary.PrintString` (`KismetStringLibrary.Concat_StrStr` (`KismetStringLibrary.Conv_IntToString` _array_index) " " (`KismetStringLibrary.Conv_NameToString` _name) "=" (`KismetStringLibrary.Conv_IntToString` _quantity)))))

(fn `LoadInventoryData`
  (params (InventoryData :type "Array of /Game/CosmicRestaurant/Blueprints/UI/Gaeun_Folder/Inventory/Inventory_Wanil/FSlotStructure Structure"))
  (`KismetArrayLibrary.Array_Resize` InventoryData (`KismetArrayLibrary.Array_Length` (`self.TempInventory`)))
  (for (_array_element _array_index) (`self.TempInventory`)
    (`KismetArrayLibrary.Array_Set` InventoryData _array_index _array_element)))

(fn `SaveInventoryData`
  (params (InventoryData :type "Array of /Game/CosmicRestaurant/Blueprints/UI/Gaeun_Folder/Inventory/Inventory_Wanil/FSlotStructure Structure"))
  (`KismetArrayLibrary.Array_Resize` (`self.TempInventory`) (`KismetArrayLibrary.Array_Length` InventoryData))
  (for (_array_element _array_index) InventoryData
    (`KismetArrayLibrary.Array_Set` (`self.TempInventory`) _array_index _array_element)))