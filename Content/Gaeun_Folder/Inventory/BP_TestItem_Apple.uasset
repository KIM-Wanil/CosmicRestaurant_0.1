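; BP_TestItem_Apple is a test inventory item actor for an apple that the player can remove by pressing F.
; Overlapping its Box sets IsRange and enables player input, so F destroys the actor; nothing resets the flag or adds to an inventory.
; LookAt looks up the ItemDataCom item ID in its data table and returns a "Find Item" text with the name.
; The InteractItem event is empty.
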(event `/Game/Gaeun_Folder/Inventory/InteractInterface.InteractItem`
  (params (PlayerCharacter :type "/Game/CosmicRestaurant/Blueprints/Character/BP_CRAdventureCharacter Object Reference")))

(event `Key|F`
  (params (Key :type "Key Structure"))
  (:`Pressed`
    (if (stale `self.Box.OnComponentBeginOverlap` _output_get)
      (`self.K2_DestroyActor`))))

(event `self.Box.OnComponentBeginOverlap`
  (params (OverlappedComponent :type "PrimitiveComponent Object Reference") (OtherActor :type "Actor Object Reference") (OtherComp :type "PrimitiveComponent Object Reference") (OtherBodyIndex :type Integer) (bFromSweep :type Boolean) (SweepResult :type "HitResult Structure (by ref)"))
  (bind _output_get (set `self.IsRange?` true))
  (`self.EnableInput` (`GameplayStatics.GetPlayerController` 0)))

(fn `LookAt`
  (returns (Message :type Text))
  (bind (_itemid_datatable _itemid_rowname) (break `DataTableRowHandle` (`/Game/Gaeun_Folder/Inventory/ItemDataCom.ItemID` (`self.ItemDataCom`))))
  (bind _returnvalue (`|GetDataTableRow` _itemid_datatable _itemid_rowname) ; 데이터 테이블에서 데이터 가져오기
    (:`then`
      (return (`|FormatText` "Find Item {item}" (`.Name_6_D913827C46689150884B4D8B238D4E53` (break `/Game/Gaeun_Folder/Inventory/FItemStructure` _returnvalue)))))))

(fn `UserConstructionScript`)