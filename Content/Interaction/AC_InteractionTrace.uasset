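; Actor component that detects which interaction area the player's camera is looking at and toggles that area's focus.
; Each tick it line-traces forward from the camera on the Visibility channel, reacting to hits only when the hit actor changes.
; Exact class checks accept Box or CustomShape areas, which are cast to the master class and focused.
; Moving to another target or hitting nothing unfocuses the previous area.
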(event `self.ReceiveTick`
  (params (DeltaSeconds :type "Float (single-precision)"))
  (`self.Trace`))

(fn `Trace`
  (bind _returnvalue (`GameplayStatics.GetPlayerCameraManager` 0))
  (bind _returnvalue_2 (`Actor.K2_GetActorLocation` _returnvalue))
  (bind (_outhit _returnvalue_3) (`KismetSystemLibrary.LineTraceSingle` _returnvalue_2 (+ _returnvalue_2 (* (`KismetMathLibrary.GetForwardVector` (`Actor.K2_GetActorRotation` _returnvalue)) (`self.Length`))) "TraceTypeQuery1"))
  (if _returnvalue_3
    (bind (_bblockinghit _binitialoverlap _time _distance _location _impactpoint _normal _impactnormal _physmat _hitactor) (`GameplayStatics.BreakHitResult` _outhit))
    (if (!= (`self.FocusedActor`) _hitactor)
      (set `self.FocusedActor` _hitactor)
      (`/Engine/EditorBlueprintResources/StandardMacros.IsValid` _hitactor
        (:`Is Valid`
          (bind _returnvalue_4 (`GameplayStatics.GetObjectClass` _hitactor))
          (`self.Traceinteraction Area` (or (== _returnvalue_4 "/Game/Interaction/InteractionArea/BP_InteractionAreas_Box.BP_InteractionAreas_Box_C") (== _returnvalue_4 "/Game/Interaction/InteractionArea/BP_InteractionAreas_CustomShape.BP_InteractionAreas_CustomShape_C"))))))
    (else
      (`self.Traceinteraction Area` false))))

(fn `Traceinteraction Area`
  (params (Trace :type Boolean))
  (bind _focusedinteractionarea (`self.FocusedInteractionArea`))
  (if Trace
    (if (`self.IsTracingInteractionArea`)
      (`/Game/Interaction/InteractionArea/BP_InteractionAreas_Master.ToggleFocus` (`self.FocusedInteractionArea`) false))
    (bind _asbp_interaction_areas_master (cast `/Game/Interaction/InteractionArea/BP_InteractionAreas_Master` (`self.FocusedActor`)))
    (bind _output_get (set `self.FocusedInteractionArea` _asbp_interaction_areas_master))
    (`/Game/Interaction/InteractionArea/BP_InteractionAreas_Master.ToggleFocus` _output_get true)
    (set `self.IsTracingInteractionArea` true)
    (elif (`self.IsTracingInteractionArea`)
      (set `self.IsTracingInteractionArea` false)
      (`/Engine/EditorBlueprintResources/StandardMacros.IsValid` _focusedinteractionarea
        (:`Is Valid`
          (`/Game/Interaction/InteractionArea/BP_InteractionAreas_Master.ToggleFocus` _focusedinteractionarea false)
          ;[1 1 1] 포커스 되는게 없으면 둘다 Null
          (set `self.FocusedActor` null)
          (set `self.FocusedInteractionArea` null))))))